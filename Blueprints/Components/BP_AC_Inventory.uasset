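; Inventory component holding item slots, sized to the container size unless it is a shop, plus a hotbar that references slots by index.
; AddItem tops up partial stacks before taking an empty slot, notifying client and HUD through call events.
; SwapItem, wrapped by SV_SwapItem, merges matching stacks or swaps slots, then broadcasts the change.
; Helpers bind the inventory widget, update hotbar widgets and spawn world or owned item actors from data-table rows.
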(event Custom|SV_SwapItem
  (params (FirstIndex :type Integer) (SecondIndex :type Integer))
  (CallFunction|SwapItem FirstIndex SecondIndex))

(event EventBeginPlay
  (if (not (Variables|Default|GetisShop))
    (CallFunction|InitSetSize)))

(fn InitSetSize
  (Utilities|Array|Resize (Variables|Default|GetData_Item) (Variables|Default|GetContainerSize)))

(fn InitWidgetItems
  (bind _foundwidgets (Widget|GetAllWidgetsOfClass "/Game/Blueprints/Widgets/WBP_GamePlay.WBP_GamePlay_C" true))
  (bind _output_get (Variables|Default|SetWBP%20GamePlay (Utilities|Array|Get(acopy) _foundwidgets)))
  (bind _output_get_2 (Variables|Default|SetWBP%20Inventory (Variables|/Game/Blueprints/Widgets/WBP_GamePlay.WBP_GamePlay_C|GetWBP_Inventory _output_get)))
  (Default|InitWBPInventory _output_get_2 self))

(fn IsEmptySlot
  (params (S_Item__Attribute :type S%20Item%20Attribute%20Structure%20%28by%20ref%29))
  (bind _table (Utilities|Struct|BreakS_Item__Attribute S_Item__Attribute))
  (return (== (.RowName (Utilities|Struct|BreakDataTableRowHandle _table)) "") _table))

(fn FindASlotHasNameandNoFull
  (params (Name :type Name) (Max :type Integer))
  (for (_array_element _array_index) (Variables|Default|GetData_Item)
    (if (and (== Name (.rowname (.Table (Utilities|Struct|BreakS_Item__Attribute _array_element)))) (< (.Quantity (Utilities|Struct|BreakS_Item__Attribute _array_element)) Max))
      (return (.Quantity (Utilities|Struct|BreakS_Item__Attribute _array_element)) _array_index)))
  (return 0 -1))

(fn GetEmptySlots
  (for (_array_element _array_index) (Variables|Default|GetData_Item)
    (if (.Empty (CallFunction|IsEmptySlot _array_element))
      (Utilities|Array|Add (LocalVariables|GetI) _array_index)))
  (return (LocalVariables|GetI)))

(fn GetAEmptySlot
  (for (_array_element _array_index) (Variables|Default|GetData_Item)
    (if (.Empty (CallFunction|IsEmptySlot _array_element))
      (return (.Empty (CallFunction|IsEmptySlot _array_element)) _array_index))))

(fn RemoveItem
  (params (Slot :type Integer))
  (Utilities|Array|Insert :TargetArray (Variables|Default|GetData_Item) :Index Slot))

(fn SwapItem
  (params (FirstIndex :type Integer) (SecondIndex :type Integer))
  (LocalVariables|Set1 FirstIndex)
  (LocalVariables|Set2 SecondIndex)
  (Utilities|FlowControl|Sequence
    (:then_0
      (if (== (.rowname (.Table (Utilities|Struct|BreakS_Item__Attribute (Utilities|Array|Get(acopy) (Variables|Default|GetData_Item) (LocalVariables|Get1))))) (.rowname (.Table (Utilities|Struct|BreakS_Item__Attribute (Utilities|Array|Get(acopy) (Variables|Default|GetData_Item) (LocalVariables|Get2))))))
        (if (or (== (.Quantity (Utilities|Struct|BreakS_Item__Attribute (Utilities|Array|Get(acopy) (Variables|Default|GetData_Item) (LocalVariables|Get1)))) (.MaxStack (Utilities|Struct|BreakS_Item__Attribute (Utilities|Array|Get(acopy) (Variables|Default|GetData_Item) (LocalVariables|Get1))))) (== (.Quantity (Utilities|Struct|BreakS_Item__Attribute (Utilities|Array|Get(acopy) (Variables|Default|GetData_Item) (LocalVariables|Get2)))) (.MaxStack (Utilities|Struct|BreakS_Item__Attribute (Utilities|Array|Get(acopy) (Variables|Default|GetData_Item) (LocalVariables|Get2))))))
          (Utilities|Array|Swap (Variables|Default|GetData_Item) (LocalVariables|Get1) (LocalVariables|Get2) :!label _label)
          (elif (>= (+ (.Quantity (Utilities|Struct|BreakS_Item__Attribute (Utilities|Array|Get(acopy) (Variables|Default|GetData_Item) (LocalVariables|Get1)))) (.Quantity (Utilities|Struct|BreakS_Item__Attribute (Utilities|Array|Get(acopy) (Variables|Default|GetData_Item) (LocalVariables|Get2))))) (.MaxStack (Utilities|Struct|BreakS_Item__Attribute (Utilities|Array|Get(acopy) (Variables|Default|GetData_Item) (LocalVariables|Get1)))))
            (Utilities|Struct|SetmembersinS_Item__Attribute (Utilities|Array|Get(acopy) (Variables|Default|GetData_Item) (LocalVariables|Get2)))
            (Utilities|Struct|SetmembersinS_Item__Attribute (Utilities|Array|Get(acopy) (Variables|Default|GetData_Item) (LocalVariables|Get1)) (- (+ (.Quantity (Utilities|Struct|BreakS_Item__Attribute (Utilities|Array|Get(acopy) (Variables|Default|GetData_Item) (LocalVariables|Get1)))) (.Quantity (Utilities|Struct|BreakS_Item__Attribute (Utilities|Array|Get(acopy) (Variables|Default|GetData_Item) (LocalVariables|Get2))))) (.MaxStack (Utilities|Struct|BreakS_Item__Attribute (Utilities|Array|Get(acopy) (Variables|Default|GetData_Item) (LocalVariables|Get1))))))
            (else
              (Utilities|Struct|SetmembersinS_Item__Attribute (Utilities|Array|Get(acopy) (Variables|Default|GetData_Item) (LocalVariables|Get2)) (+ (.Quantity (Utilities|Struct|BreakS_Item__Attribute (Utilities|Array|Get(acopy) (Variables|Default|GetData_Item) (LocalVariables|Get1)))) (.Quantity (Utilities|Struct|BreakS_Item__Attribute (Utilities|Array|Get(acopy) (Variables|Default|GetData_Item) (LocalVariables|Get2))))))
              (Utilities|Array|Insert :TargetArray (Variables|Default|GetData_Item) :Index (LocalVariables|Get1)))))
        (else
          (goto _label))))
    (:then_1
      (Default|CallOnItemsSwapped (LocalVariables|Get1) (LocalVariables|Get2)))))

(fn AddItem
  (params (Item :type S%20Item%20Attribute%20Structure%20%28by%20ref%29))
  (bind (_quantity _maxstack) (Utilities|Struct|BreakS_Item__Attribute Item))
  (bind (_empty _table) (CallFunction|IsEmptySlot Item))
  (if (not _empty)
    (LocalVariables|SetName (Utilities|Struct|BreakDataTableRowHandle _table))
    (bind _output_get (LocalVariables|SetL_Quantity _quantity))
    (bind _output_get_2 (LocalVariables|SetRemaining _output_get))
    (LocalVariables|SetL_MaxStack _maxstack)
    (Default|CallShowAddHud _table _output_get_2)
    (if (!= _maxstack 0)
      ;[0.09306 0.5417 0] Stack
      (bind (_quantity_2 _index) (CallFunction|FindASlotHasNameandNoFull (LocalVariables|GetName) (LocalVariables|GetL_MaxStack) :!label _label))
      (if (!= _index -1)
        (LocalVariables|SetRemaining (- (LocalVariables|GetL_Quantity) (- (LocalVariables|GetL_MaxStack) _quantity_2)))
        (bind _structout (Utilities|Struct|SetmembersinS_Item__Attribute (Utilities|Array|Get(acopy) (Variables|Default|GetData_Item) _index) (Math|Integer|SelectInt (LocalVariables|GetL_MaxStack) (+ _quantity_2 (LocalVariables|GetL_Quantity)) (>= (+ _quantity_2 (LocalVariables|GetL_Quantity)) (LocalVariables|GetL_MaxStack)))))
        (if (> (LocalVariables|GetRemaining) 0)
          (Default|CallEDAddItemClient _structout _index)
          (goto _label)
          (else
            (Default|CallEDAddItemClient _structout _index)
            (return true)))
        (else
          (bind (_empty_2 _index_2) (CallFunction|GetAEmptySlot))
          (if _empty_2
            (bind _structout_2 (Utilities|Struct|SetmembersinS_Item__Attribute Item (Math|Integer|SelectInt (LocalVariables|GetL_Quantity) (LocalVariables|GetRemaining) (== (LocalVariables|GetRemaining) (LocalVariables|GetL_Quantity)))))
            (Utilities|Array|SetArrayElem (Variables|Default|GetData_Item) _index_2 _structout_2)
            (Default|CallEDAddItemClient _structout_2 _index_2)
            (return true)
            (else
              (return false)))))
      (else
        ;[1 0 0] NoStack
        (bind (_empty_3 _index_3) (CallFunction|GetAEmptySlot))
        (if _empty_3
          (Utilities|Array|SetArrayElem (Variables|Default|GetData_Item) _index_3 Item)
          (Default|CallEDAddItemClient Item _index_3)
          (return true)
          (else
            (return false)))))))

(fn SetItemtoHotBar
  (params (ItemSlot :type Integer) (NumKey :type Integer))
  (bind _data_item (Variables|Default|GetData_Item))
  (bind _data_hotbar (Variables|Default|GetData_Hotbar))
  (bind _output (Utilities|Array|Get(acopy) _data_item ItemSlot))
  (bind _table (Utilities|Struct|BreakS_Item__Attribute _output))
  (if (!= NumKey -1)
    (if (Math|Boolean|ANDBoolean (not (Utilities|Array|ContainsItem _data_hotbar ItemSlot)) (or (Utilities|IsValid (.datatable _table)) (!= (.rowname _table) "")) (Utilities|Array|IsNotEmpty _data_hotbar))
      (if (== (Utilities|Array|Get(acopy) (Variables|Default|GetData_Hotbar) NumKey) -1)
        (Utilities|Array|SetArrayElem (Variables|Default|GetData_Hotbar) NumKey ItemSlot)
        (return NumKey)))))

(fn SpawnItem
  (params (D :type Data%20Table%20Row%20Handle%20Structure) (Location :type Transform) (Amount :type Integer))
  (bind _returnvalue (Utilities|GetDataTableRow (.datatable D) (.rowname D))
    (:then
      (if (Utilities|IsValidClass (.Class (Utilities|Struct|BreakS_Item__Info _returnvalue)))
        (Game|SpawnActorfromClass :Class (.Class (Utilities|Struct|BreakS_Item__Info _returnvalue)) :SpawnTransform Location :CollisionHandlingOverride "Undefined" :Instigator 0)
        (else
          (Game|SpawnActorfromClass "/Game/EasySurvivalRPG/Blueprints/InteractionObjects/Items/BP_Item.BP_Item_C" Location "Undefined" 0 (.Table (Utilities|Struct|BreakS_Item__Info _returnvalue)) Amount -1 1e+02 -1.0 true true false 0))))))

(fn SpawnItemAttach
  (params (Table :type Data%20Table%20Row%20Handle%20Structure) (Amount :type Integer) (PlayerController :type Player%20Controller%20Object%20Reference))
  (bind _returnvalue (Utilities|GetDataTableRow (.datatable Table) (.rowname Table))
    (:then
      (if (Utilities|IsValidClass (.Class (Utilities|Struct|BreakS_Item__Info _returnvalue)))
        (bind _returnvalue_2 (Game|SpawnActorfromClass (.Class (Utilities|Struct|BreakS_Item__Info _returnvalue)) (Math|Transform|MakeTransform "0, 0, 0" "0, 0, 0" "1.000000,1.000000,1.000000") "Undefined" PlayerController (.Table (Utilities|Struct|BreakS_Item__Info _returnvalue)) (.Attach_Bone (Utilities|Struct|BreakS_Item__Info _returnvalue)) (Pawn|GetControlledPawn PlayerController)))
        (return true _returnvalue_2)))))

(fn ChecktoSpawnItem)

(fn CheckSetItemtoHotBar
  (params (Slot :type Integer) (Icon :type Texture%202D%20Object%20Reference) (Quantity :type Integer))
  (bind _data_hotbar (Variables|Default|GetData_HotBar))
  (bind _returnvalue (Utilities|Array|FindItem _data_hotbar -1))
  (if (!= _returnvalue -1)
    (bind _numkey_ (HotBar|SetItemtoHotBar Slot _returnvalue))
    (if (!= _numkey_ -1)
      (bind _wbp_gameplay (Variables|Default|GetWBP%20GamePlay)
        (:then
          (bind _array_element (Utilities|Array|ForEachLoopwithBreak (Class|PanelWidget|GetAllChildren (Variables|/Game/Blueprints/Widgets/Hotbar/WBP_Hotbar_Main.WBP_Hotbar_Main_C|GetList (Variables|/Game/Blueprints/Widgets/WBP_GamePlay.WBP_GamePlay_C|GetWBP_Hotbar_Main _wbp_gameplay))) :!label _label)
            (:LoopBody
              (bind _aswbp_hotbar (Utilities|Casting|CastToWBP_Hotbar _array_element))
              (if (== (Variables|/Game/Blueprints/Widgets/Hotbar/WBP_Hotbar.WBP_Hotbar_C|GetNumber _aswbp_hotbar) _numkey_)
                (Default|Change _aswbp_hotbar Icon (Variables|/Game/Blueprints/Widgets/Hotbar/WBP_Hotbar.WBP_Hotbar_C|GetNumber _aswbp_hotbar) Quantity)
                (goto _label Break)))))
        (:else)))))