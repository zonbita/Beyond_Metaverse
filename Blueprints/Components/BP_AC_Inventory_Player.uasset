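; Player inventory component that mirrors item data to the player's inventory widget.
; On BeginPlay it initializes hotbar data and binds to add and swap delegates, whose handlers forward to OC events that update the DataItem array.
; Changed slots are refreshed in the widget with a data table icon and quantity, or zero quantity when empty.
; After a short delay, the server seeds test items from ItemTable.
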(event Custom|OC_SwapItem
  (params (Slot1 :type Integer) (Slot2 :type Integer))
  (bind _data_item (Variables|Default|GetData_Item))
  (Utilities|Array|Swap _data_item Slot1 Slot2)
  (Utilities|FlowControl|Sequence
    (:then_0
      (CallFunction|SetInfoSlot Slot1 (Utilities|Array|Get(acopy) _data_item Slot1)))
    (:then_1
      (CallFunction|SetInfoSlot Slot2 (Utilities|Array|Get(acopy) _data_item Slot2)))))

(event Custom|On_ItemsSwapped_Event
  (params (Slot1 :type Integer) (Slot2 :type Integer))
  (CallFunction|OCSwapItem Slot1 Slot2))

(event Custom|OC_AddItem
  (params (Att :type S%20Item%20Attribute%20Structure) (Slot :type Integer))
  (Utilities|Array|SetArrayElem (Variables|Default|GetData_Item) Slot Att)
  (CallFunction|SetInfoSlot Slot Att))

(event Custom|ED_AddItem_Client_Event
  (params (Attr :type S%20Item%20Attribute%20Structure) (Slot :type Integer))
  (CallFunction|OCAddItem Attr Slot))

(event EventBeginPlay
  (|CallParentFunction)
  (Utilities|FlowControl|Sequence
    (:then_0
      (Class|ACInventory|InitDataHotBar)
      (EventDispatchers|AssignEDAddItemClient (delegate Custom|ED_AddItem_Client_Event))
      (EventDispatchers|AssignOnItemsSwapped (delegate Custom|On_ItemsSwapped_Event)))
    (:then_1
      (Utilities|FlowControl|Delay 2.0)
      (if (Networking|IsServer)
        (CallFunction|TestADd)))))

(fn SetInfoSlot
  (params (Slot :type Integer) (Attribute :type S%20Item%20Attribute%20Structure%20%28by%20ref%29))
  (bind (_table _quantity) (Utilities|Struct|BreakS_Item__Attribute Attribute))
  (Utilities|IsValid (.datatable _table)
    (:Is%20Valid
      (bind _wbp_inventory (Variables|Default|GetWBP%20Inventory)
        (:then
          (bind _returnvalue (Utilities|GetDataTableRow (.datatable _table) (.rowname _table))
            (:then
              (Default|SetInfoASlot _wbp_inventory Slot (Utilities|Struct|BreakS_Item__Info _returnvalue) _quantity))))
        (:else)))
    (:Is%20Not%20Valid
      (bind _wbp_inventory_2 (Variables|Default|GetWBP%20Inventory)
        (:then
          (Default|SetInfoASlot _wbp_inventory_2 Slot))
        (:else)))))

(fn TestADd
  (for _array_element (Variables|Default|GetItem%20Table)
    (bind _returnvalue (Utilities|GetDataTableRow (.datatable _array_element) (.rowname _array_element))
      (:then
        (CallFunction|AddItem (Utilities|Struct|BreakS_Item__Info _returnvalue))))))