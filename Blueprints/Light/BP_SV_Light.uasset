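; Configurable light actor that can act as a point, rect or spot light.
; The construction script adds the light component selected by TypeNum, defaulting to point, and attaches it to the static mesh.
; BeginPlay applies intensity, attenuation radius, shadow casting and color through setters that cast the stored component to shared light base classes.
; SetSourceRadius is also called but does nothing, as its type-switch logic is disconnected.
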(event EventBeginPlay
  (CallFunction|SetIntensity (Variables|Default|GetNew%20Intensity))
  (CallFunction|SetAttenuationRadius (Variables|Default|GetAttenuation%20Radius))
  (CallFunction|SetSourceRadius (Variables|Default|GetSource%20Radius))
  (CallFunction|SetCastShadows (Variables|Default|GetEnable))
  (CallFunction|SetColor (Variables|Default|GetNew%20Light%20Color)))

(fn ConstructionScript
  (bind _staticmesh (Variables|Default|GetStaticMesh))
  (switch int (Variables|Default|GetTypeNum)
    (:Default
      (bind _returnvalue (AddComponent|AddPointLightComponent false :!label _label))
      (Variables|Default|SetComponent _returnvalue)
      (Transformation|AttachComponentToComponent _returnvalue _staticmesh "None" "KeepRelative" "KeepRelative" "KeepRelative" true))
    (:0
      (goto _label))
    (:1
      (bind _returnvalue_2 (AddComponent|AddRectLightComponent false))
      (Variables|Default|SetComponent _returnvalue_2)
      (Transformation|AttachComponentToComponent _returnvalue_2 _staticmesh "None" "KeepRelative" "KeepRelative" "KeepRelative" true))
    (:2
      (bind _returnvalue_3 (AddComponent|AddSpotLightComponent false))
      (Variables|Default|SetComponent _returnvalue_3)
      (Transformation|AttachComponentToComponent _returnvalue_3 _staticmesh "None" "KeepRelative" "KeepRelative" "KeepRelative" true))))

(fn SetIntensity
  (params (NewIntensity :type Float%20%28single-precision%29))
  (bind _component (Variables|Default|GetComponent)
    (:then
      (bind _aslocal_light_component (Utilities|Casting|CastToLocalLightComponent _component))
      (Rendering|Components|Light|SetIntensity _aslocal_light_component NewIntensity))
    (:else)))

(fn SetAttenuationRadius
  (params (NewRadius :type Float%20%28single-precision%29))
  (bind _component (Variables|Default|GetComponent)
    (:then
      (bind _aslocal_light_component (Utilities|Casting|CastToLocalLightComponent _component))
      (Rendering|Lighting|SetAttenuationRadius _aslocal_light_component NewRadius))
    (:else)))

(fn SetSourceRadius
  (params (Source%20Radius :type Float%20%28single-precision%29)))

(fn SetCastShadows
  (params (Enable :type Boolean))
  (bind _component (Variables|Default|GetComponent)
    (:then
      (bind _aslocal_light_component (Utilities|Casting|CastToLocalLightComponent _component))
      (Rendering|Components|Light|SetCastShadows _aslocal_light_component Enable))
    (:else)))

(fn SetColor
  (params (NewLightColor :type Linear%20Color%20Structure))
  (bind _component (Variables|Default|GetComponent)
    (:then
      (bind _aslight_component (Utilities|Casting|CastToLightComponent _component))
      (Rendering|Components|Light|SetLightColor _aslight_component NewLightColor true))
    (:else)))