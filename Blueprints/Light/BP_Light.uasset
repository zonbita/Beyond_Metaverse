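; BP_Light is a configurable light actor that can act as a point, rect or spot light.
; The construction script adds the light component chosen by TypeNum, defaulting to point, attaches it to StaticMesh and stores it in Component.
; Setter and getter functions cast Component to expose intensity, color, attenuation radius, shadow casting and source radius.
; Source radius applies only to point and spot lights, and reads as zero for rect lights.
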(fn ConstructionScript
  (bind _staticmesh (Variables|Default|GetStaticMesh))
  (switch int (Variables|Default|GetTypeNum)
    (:Default
      (bind _returnvalue (AddComponent|AddPointLightComponent false :!label _label))
      (Variables|Default|SetComponent _returnvalue)
      (Transformation|AttachComponentToComponent _returnvalue _staticmesh "None" "KeepRelative" "KeepRelative" "KeepRelative" true))
    (:0
      (goto _label))
    (:1
      (bind _returnvalue_2 (AddComponent|AddRectLightComponent false))
      (Variables|Default|SetComponent _returnvalue_2)
      (Transformation|AttachComponentToComponent _returnvalue_2 _staticmesh "None" "KeepRelative" "KeepRelative" "KeepRelative" true))
    (:2
      (bind _returnvalue_3 (AddComponent|AddSpotLightComponent false))
      (Variables|Default|SetComponent _returnvalue_3)
      (Transformation|AttachComponentToComponent _returnvalue_3 _staticmesh "None" "KeepRelative" "KeepRelative" "KeepRelative" true))))

(fn SetIntensity
  (params (NewIntensity :type Float%20%28single-precision%29))
  (bind _component (Variables|Default|GetComponent)
    (:then
      (bind _aslight_component (Utilities|Casting|CastToLightComponent _component))
      (Rendering|Components|Light|SetIntensity _aslight_component NewIntensity))
    (:else)))

(fn SetAttenuationRadius
  (params (NewRadius :type Float%20%28single-precision%29))
  (bind _component (Variables|Default|GetComponent)
    (:then
      (bind _aslocal_light_component (Utilities|Casting|CastToLocalLightComponent _component))
      (Rendering|Lighting|SetAttenuationRadius _aslocal_light_component NewRadius))
    (:else)))

(fn SetSourceRadius
  (params (Source%20Radius :type Float%20%28single-precision%29))
  (bind _component (Variables|Default|GetComponent))
  (switch int (Variables|Default|GetTypeNum)
    (:Default
      (bind _aspoint_light_component (Utilities|Casting|CastToPointLightComponent _component :!label _label)))
    (:0
      (goto _label))
    (:2
      (bind _aspoint_light_component_2 (Utilities|Casting|CastToPointLightComponent _component))))
  (Class|PointLightComponent|SetSourceRadius _aspoint_light_component Source%20Radius))

(fn SetCastShadows
  (params (Enable :type Boolean))
  (bind _component (Variables|Default|GetComponent)
    (:then
      (bind _aslocal_light_component (Utilities|Casting|CastToLocalLightComponent _component))
      (Rendering|Components|Light|SetCastShadows _aslocal_light_component Enable))
    (:else)))

(fn GetValues
  (bind _component (Variables|Default|GetComponent)
    (:then
      (bind _aslocal_light_component (Utilities|Casting|CastToLocalLightComponent _component))
      (bind _aslight_component (Utilities|Casting|CastToLightComponent _component))
      (return (Variables|/Script/Engine.LightComponentBase|GetIntensity _aslocal_light_component) (Variables|/Script/Engine.LocalLightComponent|GetAttenuationRadius _aslocal_light_component) (Math|Float|SelectFloat (Variables|/Script/Engine.PointLightComponent|GetSourceRadius (.AsPoint%20Light%20Component (Utilities|Casting|CastToPointLightComponent _component))) 0.0 (.bSuccess (Utilities|Casting|CastToPointLightComponent _component))) (Variables|/Script/Engine.LightComponentBase|GetCastShadows _aslocal_light_component) (Rendering|Components|Light|GetLightColor _aslight_component)))
    (:else)))

(fn SetColor
  (params (NewLightColor :type Linear%20Color%20Structure))
  (bind _component (Variables|Default|GetComponent)
    (:then
      (bind _aslight_component (Utilities|Casting|CastToLightComponent _component))
      (Rendering|Components|Light|SetLightColor _aslight_component NewLightColor true))
    (:else)))