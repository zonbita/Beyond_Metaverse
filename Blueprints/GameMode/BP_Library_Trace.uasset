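; Blueprint function library of camera-based trace helpers that find what player 0 is looking at.
; Both functions cast from the camera manager's location along its forward vector over a given range and return the hit and a success flag.
; LTrace runs a Visibility line trace with timed debug drawing.
; LTraceObjects runs a sphere trace with a given radius against supplied object types, without debug drawing.
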(fn LTrace
  (params (Range :type Integer))
  (bind _returnvalue (Game|GetPlayerCameraManager 0))
  (bind _returnvalue_2 (Camera|GetCameraLocation _returnvalue))
  (bind (_outhit _returnvalue_3) (Collision|LineTraceByChannel 0 _returnvalue_2 (+ _returnvalue_2 (* (Transformation|GetActorForwardVector _returnvalue) Range)) "TraceTypeQuery1" false 0 "ForDuration"))
  (return _outhit _returnvalue_3))

(fn LTraceObjects
  (params (Radius :type Float%20%28single-precision%29) (Range :type Integer) (ObjectTypes :type Array%20of%20EObjectTypeQuery%20Enums :default "ObjectTypeQuery1"))
  (bind _returnvalue (Game|GetPlayerCameraManager 0))
  (bind _returnvalue_2 (Camera|GetCameraLocation _returnvalue))
  (bind (_outhit _returnvalue_3) (Collision|SphereTraceForObjects 0 _returnvalue_2 (+ _returnvalue_2 (* (Transformation|GetActorForwardVector _returnvalue) Range)) Radius ObjectTypes false 0 "None"))
  (return _outhit _returnvalue_3))