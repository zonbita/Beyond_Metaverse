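; Blueprint helper library for reading light settings and cycling character skins.
; GetValuesLight matches property names in one array to string values in a parallel array, converting them to type, intensity, attenuation and source radius, shadow casting and color.
; SetSkinIDCharacter steps an ID forward or back by a boolean, wrapping at either end of ArraySkinTable, and returns the resulting class and ID.
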(fn GetValuesLight
  (params (A :type Array%20of%20Strings) (B :type Array%20of%20Strings))
  (for (_array_element _array_index) A
    (switch string _array_element
      (:Type
        (LocalVariables|SetT (Math|Conversions|ToInteger(Byte) (Utilities|Array|Get(acopy) B _array_index))))
      (:Intensity
        (LocalVariables|Set11 (Math|Conversions|ToFloat(Integer) (Utilities|Array|Get(acopy) B _array_index))))
      (:AttenuationRadius
        (LocalVariables|Set12 (Math|Conversions|ToFloat(Integer) (Utilities|Array|Get(acopy) B _array_index))))
      (:SourceRadius
        (LocalVariables|Set13 (Math|Conversions|ToFloat(Integer) (Utilities|Array|Get(acopy) B _array_index))))
      (:CastShadows
        (LocalVariables|SetC (Utilities|Enum|Equal(Enum) (Utilities|Array|Get(acopy) B _array_index) "true")))
      (:Color
        (LocalVariables|SetColor (.OutConvertedColor (Math|Conversions|ToColor(LinearColor) (Utilities|Array|Get(acopy) B _array_index)))))))
  (return (LocalVariables|GetT) (LocalVariables|Get11) (LocalVariables|Get12) (LocalVariables|Get13) (LocalVariables|GetC) (LocalVariables|GetColor)))

(fn SetSkinIDCharacter
  (params (+ :type Boolean) (id :type Integer))
  (bind _pawn (CallFunction|ArraySkinTable))
  (bind _returnvalue (+ id 1))
  (bind _returnvalue_2 (- id 1))
  (bind _returnvalue_3 (Utilities|Array|LastIndex _pawn))
  (bind _returnvalue_4 (< _returnvalue_2 0))
  (bind _returnvalue_5 (Math|Integer|SelectInt _returnvalue_3 _returnvalue_2 _returnvalue_4))
  (bind _returnvalue_6 (> _returnvalue _returnvalue_3))
  (bind _returnvalue_7 (Math|Integer|SelectInt 0 _returnvalue _returnvalue_6))
  (bind _returnvalue_8 (Math|Integer|SelectInt _returnvalue_7 _returnvalue_5 +))
  (bind _returnvalue_9 (Math|Integer|Clamp(Integer) _returnvalue_8 0 _returnvalue_3))
  (return (Utilities|Array|Get(acopy) _pawn _returnvalue_9) _returnvalue_9))

(fn ArraySkinTable
  (return (LocalVariables|GetP)))