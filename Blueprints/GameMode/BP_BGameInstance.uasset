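; BP_BGameInstance is a game instance that automatically connects non-dedicated-server instances to a server on startup.
; Init calls ConnecttoServer, which waits a very short delay and then switches on the current level name.
; The Client and Lobby levels each run an "open" console command built from the IP variable, with Lobby targeting port 7000 and Client specifying no port.
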(event Custom|Connect%20to%20Server
  (bind _ip (Variables|Default|GetIP))
  (Utilities|FlowControl|Delay 0.01)
  (bind _returnvalue (Game|GetCurrentLevelName true))
  (switch string _returnvalue
    (:Client
      (Development|ExecuteConsoleCommand (Utilities|String|ToString(Text) (Utilities|Text|FormatText "open {ip}" _ip)) 0))
    (:Lobby
      (Development|ExecuteConsoleCommand (Utilities|String|ToString(Text) (Utilities|Text|FormatText "open {ip}:7000" _ip)) 0))))

(event EventInit
  (if (not (Networking|IsDedicatedServer))
    (CallFunction|ConnecttoServer)))