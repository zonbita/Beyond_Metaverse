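; BP_SocketServer periodically reports player names and pawn locations to a Socket.IO server.
; A looping timer started on BeginPlay runs Call every two seconds, gathering data from GameState's PlayerArray into parallel name and location string arrays.
; These are wrapped in JSON keyed by the current level name and emitted as a "Statistics" event.
; The graph never clears the arrays, so entries accumulate across calls.
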(event EventBeginPlay
  (Utilities|Time|SetTimerbyFunctionName 0 "call" 2.0 true))

(fn ConstructionScript)

(fn Call
  (bind _returnvalue (Game|GetGameState))
  (Utilities|IsValid _returnvalue
    (:Is%20Valid
      (for _array_element (Variables|/Script/Engine.GameStateBase|GetPlayerArray _returnvalue)
        (Utilities|IsValid (PlayerState|GetPawn _array_element)
          (:Is%20Valid
            (bind _returnvalue_2 (Utilities|Array|Add (LocalVariables|GetN) (PlayerState|GetPlayerName _array_element)))
            (Utilities|Array|SetArrayElem (LocalVariables|GetL) _returnvalue_2 (Utilities|String|ToString(Vector) (Transformation|GetActorLocation (PlayerState|GetPawn _array_element))) true))))
      (Utilities|FlowControl|Sequence
        (:then_0
          (bind _returnvalue_3 (Class|SIOJsonObject|ConstructJsonObject))
          (Class|SIOJsonObject|SetStringArrayField _returnvalue_3 "Name" (LocalVariables|GetN))
          (Class|SIOJsonObject|SetStringArrayField _returnvalue_3 "Location" (LocalVariables|GetL)))
        (:then_1
          (bind _returnvalue_4 (Class|SIOJsonObject|ConstructJsonObject))
          (bind _returnvalue_5 (Game|GetCurrentLevelName true))
          (Class|SIOJsonObject|SetArrayField _returnvalue_4 _returnvalue_5 (Utilities|Array|MakeArray (Class|SIOJLibrary|ToJsonValue(JsonObject) _returnvalue_3)))
          (Class|SocketIOClientComponent|Emit (Variables|Default|GetSocketIOClient) "Statistics" (Class|SIOJLibrary|ToJsonValue(JsonObject) _returnvalue_4) "/"))))))