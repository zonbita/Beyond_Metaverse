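; BP_BGamePlay is a game mode Blueprint that spawns and possesses player characters at a PlayerStart.
; Init caches a PlayerStart found by class, running on BeginPlay and again if the reference is invalid at spawn time.
; Spawn_Character spawns BP_ThirdPersonCharacter with the given skin ID, owned and possessed by the target controller.
; PostLogin is empty, and its server-side auto-spawn logic is disconnected.
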(event Custom|Spawn_Character
  (params (IDCharacter :type Integer) (Target :type Controller%20Object%20Reference))
  (Variables|Default|GetPlayerStart
    (:then
      _)
    (:else
      (CallFunction|Init)))
  (bind _returnvalue (Game|SpawnActorfromClass "/Game/ThirdPerson/Blueprints/BP_ThirdPersonCharacter.BP_ThirdPersonCharacter_C" (Transformation|GetActorTransform (Variables|Default|GetPlayerStart)) "Undefined" Target IDCharacter 0))
  (Pawn|Possess Target _returnvalue))

(event EventBeginPlay
  (CallFunction|Init))

(event EventPostLogin
  (params (NewPlayer :type Player%20Controller%20Object%20Reference)))

(fn ConstructionScript)

(fn Init
  (bind _returnvalue (Actor|GetActorOfClass "/Script/Engine.PlayerStart"))
  (Variables|Default|SetPlayerStart _returnvalue))