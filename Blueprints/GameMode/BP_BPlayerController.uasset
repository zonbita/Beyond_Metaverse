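; Player controller for a multiplayer hex-region building game, relaying requests between owning client and server.
; Client timers request nearby regions and build meshes from returned blocks; a server timer then streams each visited region's GLTF assets.
; GLTF and light edits are persisted through HexGridManager and the GLTF spawn manager, with chunk traces by player name gating placement.
; It also handles player setup, triangle placement, edit-pawn UI and inventory hotbar items.
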(event Custom|SV_Spawn_GLTF
  (params (Name :type String) (Transform :type Transform) (CTag :type Compount%20Container%20Structure))
  ;[1 0 0] Call_Spawn_GLTF
  (Utilities|CastGLTFManager)
  (bind _output_get (Variables|Default|SetTransform Transform))
  (bind (_regionname _ownername _trianglename _returnvalue) (Class|BPlayerController|TraceChunk (.Location (Math|Transform|BreakTransform _output_get)) "TraceTypeQuery3" (PlayerState|GetPlayerName (Variables|Default|GetPlayerState))))
  (if _returnvalue
    (bind _index (Class|HexGridManager|SaveARegionAsset (Variables|Default|GetHexGridManager) _regionname Name (Variables|Default|GetTransform) (Utilities|Struct|MakeAsset_Info _trianglename _ownername 1e+02 0 0) CTag))
    (bind _data (Class|BLibrary|ConvertCompoundTagstoData (Utilities|Struct|BreakCompountContainer CTag)))
    (Default|SVSpawnGLTF (Variables|Default|GetGLTF_Manager) Name _regionname (Variables|Default|GetTransform) _index (Utilities|Struct|MakeAsset_Info _trianglename _ownername 1e+02 0 0) (Utilities|Struct|MakeCompountContainer2 _data))))

(event Custom|SV_SetPlayerData
  (params (PDI :type Player%20Data%20Info%20Structure))
  (bind _returnvalue (Game|GetGameMode))
  ;[0 0.08937 1] Begin - Set Player Data
  (Class|GameModeBase|ChangeName _returnvalue self (.playername PDI) true)
  (Default|SpawnCharacter (.AsBP%20BGame%20Play (Utilities|Casting|CastToBP_BGamePlay _returnvalue)) (.idcharacter PDI) self))

(event Custom|OC_Possess_EditPawn
  (params (Edit_Pawn :type Edit%20Pawn%20Object%20Reference))
  ;[0 0.07217 1] EditPawn
  (Utilities|IsValid Edit_Pawn
    (:Is%20Valid
      (Default|FindWidget Edit_Pawn)
      (bind _widget_transform (Variables|/Game/Blueprints/Actor_Base/EditPawn.EditPawn_C|GetWidget_transform Edit_Pawn)
        (:then
          (Variables|Default|SetbShowMouseCursor true)
          (Variables|/Game/Blueprints/Widgets/RTTM_Widget.RTTM_Widget_C|SetTransformerActor _widget_transform Edit_Pawn)
          (Class|WidgetSwitcher|SetActiveWidgetIndex (Variables|/Game/Blueprints/Actor_Base/EditPawn.EditPawn_C|GetWidget%20Switcher Edit_Pawn) 1)
          (Default|SetInputMode Edit_Pawn false)
          (Class|BPlayerController|SetOwnerChunkManager Edit_Pawn (Utilities|GetPlayerName))
          (CallFunction|SetOwnerLight0 Edit_Pawn))
        (:else)))))

(event Custom|OC_Spawn_Light
  (params (SpawnTransform :type Transform) (Type :type Integer) (Intensity :type Float%20%28single-precision%29) (Attenuation%20Radius :type Float%20%28single-precision%29) (Source%20Radius :type Float%20%28single-precision%29) (Enable :type Boolean) (LinearColor :type Linear%20Color%20Structure))
  ;[0.6222 1 0] Lightning
  (CallFunction|SVSpawnLight SpawnTransform Type Intensity Attenuation%20Radius Source%20Radius Enable LinearColor))

(event Custom|SV_GetDataARegion
  (params (RegionName :type String))
  (bind _hexgridmanager (Variables|Default|GetHexGridManager))
  ;[0 0.4456 1] Region
  (Utilities|FlowControl|Sequence
    (:then_0
      (bind _returnvalue (Class|HexGridManager|FindDataOfRegion _hexgridmanager RegionName))
      (if (not (Utilities|Array|IsEmpty (.regionname _returnvalue)))
        (bind _b (Class|HexGridManager|GetBlocksARegion _hexgridmanager (Utilities|Struct|MakeRegionData (.regionname _returnvalue) (.chunkdata _returnvalue))))
        (CallFunction|OCSetBlocks (.regionname _returnvalue) _b)))
    (:then_1
      (Utilities|FlowControl|DoOnce false
        (:Completed
          (Utilities|CastGLTFManager)
          (Utilities|Time|SetTimerbyFunctionName 0 "Check_Loc_Assets" 1.0 true))))))

(event Custom|OC_CheckLoad_Assets
  (params (RegionName :type String%20%28by%20ref%29) (Array :type Array%20of%20Strings))
  ;[1 0 0] Call_Spawn_GLTF
  (Default|CheckLoadAssetGLTF (Variables|Default|GetGLTF_Manager) RegionName Array))

(event Custom|OC_SetOwnerRegion
  (params (Region :type Array%20of%20Strings))
  ;[0 0.4456 1] Region
  (bind _hexgridmanager (Variables|Default|GetHexGridManager)
    (:then
      (Class|HexGridManager|SetMyRegionUnique _hexgridmanager Region))
    (:else)))

(event Custom|SV_Remove_Light
  (params (BP%20SVLight :type BP%20SV%20Light%20Object%20Reference))
  ;[0.6222 1 0] Lightning
  (Utilities|CastHex)
  (bind _returnvalue (Class|HexGridManager|RemoveGLTFSlotfromChunkAssets (Variables|Default|GetHexGridManager) (Variables|/Game/Blueprints/Light/BP_SV_Light.BP_SV_Light_C|GetRegionName BP%20SVLight) (PlayerState|GetPlayerName (Variables|Default|GetPlayerState)) "B:Light" (Variables|/Game/Blueprints/Light/BP_SV_Light.BP_SV_Light_C|GetSlotIndex BP%20SVLight)))
  (if _returnvalue
    (Actor|DestroyActor BP%20SVLight)))

(event Custom|PC_SV_Delete_GLTF
  (params (Async%20GLTF%20Spawn :type BP%20Async%20GLTF%20Spawn%20Object%20Reference))
  ;[1 0 0] Call_Spawn_GLTF
  (Utilities|IsValid Async%20GLTF%20Spawn
    (:Is%20Valid
      (Utilities|CastHex)
      (bind _returnvalue (Class|HexGridManager|RemoveGLTFSlotfromChunkAssets (Variables|Default|GetHexGridManager) (Variables|/Game/Blueprints/Actor_Base/BP_Async_GLTF_Spawn.BP_Async_GLTF_Spawn_C|GetHexagon Async%20GLTF%20Spawn) (PlayerState|GetPlayerName (Variables|Default|GetPlayerState)) (Variables|/Game/Blueprints/Actor_Base/BP_Async_GLTF_Spawn.BP_Async_GLTF_Spawn_C|GetGLTF_Name Async%20GLTF%20Spawn) (Variables|/Game/Blueprints/Actor_Base/BP_Async_GLTF_Spawn.BP_Async_GLTF_Spawn_C|GetIndex Async%20GLTF%20Spawn)))
      (if _returnvalue
        (Actor|DestroyActor Async%20GLTF%20Spawn)))))

(event Custom|OC_Place_Hexagon
  (params (Name :type String) (Chunk :type BP%20Chunk%20Manager%20Object%20Reference) (ArrayTriangleName :type Array%20of%20Strings) (Up :type Boolean))
  ;[1 1 1] Comment
  (CallFunction|SVCheckPlaceHexagon Chunk Up Name ArrayTriangleName (select Up (Variables|/Script/BeyondOnline2.ChunkManager|GetHISM1 Chunk) (Variables|/Script/BeyondOnline2.ChunkManager|GetHISM2 Chunk))))

(event Custom|SV_CheckPlaceHexagon
  (params (BPChunk :type Chunk%20Manager%20Object%20Reference) (Up :type Boolean) (TriangleName :type String) (ArrayTriangleName :type Array%20of%20Strings) (HISM :type Hexagon%20HISM%20Object%20Reference))
  ;[1 1 1] Comment
  (bind (_n _location _returnvalue) (Class|ChunkManager|ChecktoSpawnTriangle BPChunk Up TriangleName ArrayTriangleName HISM))
  (if _returnvalue
    (Class|ChunkManager|SpawnATriangle BPChunk _n _location TriangleName HISM)))

(event Custom|SV_SendNumKey
  (params (NumKey :type Integer) (ItemSlot :type Integer))
  (bind _returnvalue (Pawn|GetControlledPawn))
  (bind _bp_ac_inventory_player (Variables|Components|GetBP_AC_Inventory_Player))
  (bind _data_item (Variables|/Game/Blueprints/Components/BP_AC_Inventory.BP_AC_Inventory_C|GetData_Item _bp_ac_inventory_player))
  (bind _output (Utilities|Array|Get(acopy) _data_item ItemSlot))
  (Utilities|IsValid _returnvalue
    (:Is%20Valid
      (bind _actors (Class|ICharacter|IGetItemUse(Message) _returnvalue))
      (Utilities|IsValid (Utilities|Array|Get(acopy) _actors NumKey)
        (:Is%20Valid
          (Class|ICharacter|ISetItemUse(Message) _returnvalue (Utilities|Array|Get(acopy) _actors NumKey) NumKey))
        (:Is%20Not%20Valid
          (Utilities|IsValid (.DataTable (Utilities|Struct|BreakDataTableRowHandle (.table _output)))
            (:Is%20Valid
              (bind (_spawn _actor) (Default|SpawnItemAttach _bp_ac_inventory_player (.table _output) 1 self))
              (if _spawn
                (bind _asitem_attach (Utilities|Casting|CastToItem_Attach _actor))
                (Class|ICharacter|ISetItemUse(Message) _returnvalue _asitem_attach NumKey)))))))))

(event Custom|OC_SetBlocks
  (params (RegionName :type String) (BlocksArray :type Array%20of%20Array%20Unit%208%20Structures))
  ;[0 0.4456 1] Region
  (Utilities|FlowControl|Sequence
    (:then_0
      (if (Utilities|Array|IsValidIndex BlocksArray)
        (bind _returnvalue (Class|HexGridManager|CLFindChunkManager (Variables|Default|GetHexGridManager) RegionName))
        (Utilities|IsValid _returnvalue
          (:Is%20Valid
            (Class|ChunkManager|CLGenerateMeshfromBlocks _returnvalue BlocksArray)
            (Utilities|Array|Add (Variables|Default|GetRegionName_Map) RegionName)))))
    (:then_1
      (Utilities|FlowControl|DoOnce false
        (:Completed
          (Variables|Default|SetisLoadMap true))))))

(event Custom|OC_Call_Save
  (params (Async%20GLTF%20Spawn :type BP%20Async%20GLTF%20Spawn%20Object%20Reference) (InTransform :type Transform%20%28by%20ref%29))
  ;[1 0 0] Call_Spawn_GLTF
  (Utilities|IsValid Async%20GLTF%20Spawn
    (:Is%20Valid
      (bind _gltf (Variables|/Game/Blueprints/Actor_Base/BP_Async_GLTF_Spawn.BP_Async_GLTF_Spawn_C|GetGLTF Async%20GLTF%20Spawn)
        (:then
          (CallFunction|SVCallSave Async%20GLTF%20Spawn InTransform (Variables|/Game/Blueprints/Actor_Base/BP_Async_GLTF.BP_Async_GLTF_C|GetColors _gltf)))
        (:else)))))

(event Custom|OC_Call_Remove_Light
  (params (BPLight :type BP%20SV%20Light%20Object%20Reference))
  ;[0.6222 1 0] Lightning
  (CallFunction|SVRemoveLight BPLight))

(event Custom|Call_Spawn_GLTF
  (params (Name :type String) (Location :type Transform) (CTag :type Compount%20Container%20Structure))
  ;[1 0 0] Call_Spawn_GLTF
  (CallFunction|SVSpawnGLTF Name Location CTag))

(event Custom|PC_Call_Delete_GLTF
  (params (Async%20GLTF%20Spawn :type BP%20Async%20GLTF%20Spawn%20Object%20Reference))
  ;[1 0 0] Call_Spawn_GLTF
  (CallFunction|PCSVDeleteGLTF Async%20GLTF%20Spawn))

(event Custom|SV_Spawn_Light
  (params (SpawnTransform :type Transform) (Type :type Integer) (Intensity :type Float%20%28single-precision%29) (Attenuation%20Radius :type Float%20%28single-precision%29) (Source%20Radius :type Float%20%28single-precision%29) (Enable :type Boolean) (LinearColor :type Linear%20Color%20Structure))
  ;[0.6222 1 0] Lightning
  (bind (_regionname _ownername _trianglename _returnvalue) (Class|BPlayerController|TraceChunk (.Location (Math|Transform|BreakTransform SpawnTransform)) "TraceTypeQuery3" (PlayerState|GetPlayerName (Variables|Default|GetPlayerState))))
  (if _returnvalue
    (bind _index (Class|HexGridManager|SaveARegionAsset (Variables|Default|GetHexGridManager) _regionname "B:Light" SpawnTransform (Utilities|Struct|MakeAsset_Info _trianglename _ownername 1e+02 0 0) (Utilities|Struct|MakeCompountContainer (Utilities|Array|MakeArray (Utilities|Struct|MakeCompountTags "B:Light" (Utilities|Map|MakeMap "Type" (Utilities|String|ToString(Integer) Type) "Intensity" (Utilities|String|ToString(Float) Intensity) "AttenuationRadius" (Utilities|String|ToString(Float) Attenuation%20Radius) "SourceRadius" (Utilities|String|ToString(Float) Source%20Radius) "CastShadows" (Utilities|String|ToString(Boolean) Enable) "Color" (Utilities|String|ToString(Integer) LinearColor)))))))
    (Game|SpawnActorfromClass "/Game/Blueprints/Light/BP_SV_Light.BP_SV_Light_C" SpawnTransform "Undefined" (Game|Player|GetPlayerPawn 0) Type Intensity Attenuation%20Radius Source%20Radius Enable LinearColor _regionname _index "" 0)))

(event Custom|SV_Call_Save
  (params (Async%20GLTF%20Spawn :type BP%20Async%20GLTF%20Spawn%20Object%20Reference) (InTransform :type Transform%20%28by%20ref%29) (Colors :type Array%20of%20Color%20Materials%20Structures))
  ;[1 0 0] Call_Spawn_GLTF
  (Utilities|IsValid Async%20GLTF%20Spawn
    (:Is%20Valid
      (Utilities|CastGLTFManager)
      (Utilities|CastHex)
      (bind (_regionname _ownername _trianglename _returnvalue) (Class|BPlayerController|TraceChunk (.Location (Math|Transform|BreakTransform InTransform)) "TraceTypeQuery3" (PlayerState|GetPlayerName (Variables|Default|GetPlayerState))))
      (if _returnvalue
        (bind (_newindex _botherchunk _returnvalue_2) (Class|HexGridManager|CustomizeARegionAsset (Variables|Default|GetHexGridManager) (Variables|/Game/Blueprints/Actor_Base/BP_Async_GLTF_Spawn.BP_Async_GLTF_Spawn_C|GetRegion Async%20GLTF%20Spawn) _regionname (Variables|/Game/Blueprints/Actor_Base/BP_Async_GLTF_Spawn.BP_Async_GLTF_Spawn_C|GetGLTF_Name Async%20GLTF%20Spawn) InTransform (Variables|/Game/Blueprints/Actor_Base/BP_Async_GLTF_Spawn.BP_Async_GLTF_Spawn_C|GetIndex Async%20GLTF%20Spawn)))
        (if _returnvalue_2
          (Utilities|FlowControl|Sequence
            (:then_0
              (Default|MCCallTransform Async%20GLTF%20Spawn InTransform))
            (:then_1
              (CallFunction|SVSetMaterialColor Async%20GLTF%20Spawn Colors :!label _label)
              (if _botherchunk
                (Variables|/Game/Blueprints/Actor_Base/BP_Async_GLTF_Spawn.BP_Async_GLTF_Spawn_C|SetIndex Async%20GLTF%20Spawn _newindex)
                (Variables|/Game/Blueprints/Actor_Base/BP_Async_GLTF_Spawn.BP_Async_GLTF_Spawn_C|SetRegion Async%20GLTF%20Spawn _regionname))))
          (else
            (goto _label)))))))

(event Custom|OC_Unpossess_EditPawn
  (params (Edit_Pawn :type Edit%20Pawn%20Object%20Reference))
  (bind _self self)
  ;[0 0.07217 1] EditPawn
  (Utilities|IsValid Edit_Pawn
    (:Is%20Valid
      (Variables|Default|SetbShowMouseCursor false)
      (Class|WidgetSwitcher|SetActiveWidgetIndex (Variables|/Game/Blueprints/Actor_Base/EditPawn.EditPawn_C|GetWidget%20Switcher Edit_Pawn))
      (Input|EnableInput (Variables|/Script/Engine.Actor|GetInstigator Edit_Pawn) _self)
      (Input|SetInputModeGameOnly _self false))))

(event Custom|OC_Widget_TransformActor
  (params (Edit_Pawn :type Edit%20Pawn%20Object%20Reference))
  ;[0 0.07217 1] EditPawn
  (Default|FindWidget Edit_Pawn))

(event Custom|OC_Location_Json
  (params (Name :type String) (Hex :type Chunk%20Data%20Structure))
  ;[0 0.08937 1] Begin - Set Player Data
  (Class|HexGridManager|CLCreateHexagon (Variables|Default|GetHexGridManager) Name Hex))

(event EventBeginPlay
  ;[0 0.08937 1] Begin - Set Player Data
  (Utilities|FlowControl|Sequence
    (:then_0
      (Utilities|CastHex)
      (Utilities|CastGLTFManager))
    (:then_1
      (if (not (Networking|IsServer))
        (CallFunction|FirstLoc)
        (Utilities|Time|SetTimerbyFunctionName 0 "Check_Loc_Json" 2.0 true 0.1)
        (Utilities|FlowControl|Delay 0.2)
        (CallFunction|GetPlayerNamefromClient)))))

(event EventEndPlay
  (params (EndPlayReason :type EEndPlayReason%20Enum :default "Destroyed"))
  (bind _returnvalue (Pawn|GetControlledPawn))
  (Utilities|IsValid _returnvalue
    (:Is%20Valid
      (bind _asbp_third_person_character (Utilities|Casting|CastToBP_ThirdPersonCharacter _returnvalue))
      (bind _editpawn (Variables|/Game/ThirdPerson/Blueprints/BP_ThirdPersonCharacter.BP_ThirdPersonCharacter_C|GetEditPawn _asbp_third_person_character)
        (:then
          (Actor|DestroyActor _editpawn))
        (:else)))))

(event EventISendNumKeytoPC
  (params (Numkey :type Integer))
  (bind _bp_ac_inventory_player (Variables|Components|GetBP_AC_Inventory_Player))
  (bind _data_hotbar (Variables|/Script/BeyondOnline2.AC_Inventory|GetData_HotBar _bp_ac_inventory_player))
  (bind _output (Utilities|Array|Get(acopy) _data_hotbar Numkey))
  (if (!= _output -1)
    (CallFunction|SVSendNumKey Numkey _output)))

(event Input|ActionEvents|InputActionInventory
  (params (Key :type Key%20Structure :default "None"))
  (bind _bp_ac_inventory_player (Variables|Components|GetBP_AC_Inventory_Player))
  (bind _wbp_gameplay (Variables|/Game/Blueprints/Components/BP_AC_Inventory.BP_AC_Inventory_C|GetWBP%20GamePlay _bp_ac_inventory_player))
  ;[1 0 0.8952] Inventory
  (:Pressed
    (bind _wbp_inventory (Variables|/Game/Blueprints/Components/BP_AC_Inventory.BP_AC_Inventory_C|GetWBP%20Inventory _bp_ac_inventory_player)
      (:then
        (Widget|SetVisibility _wbp_inventory (select (Widget|IsVisible _wbp_inventory) "Hidden" "Visible"))
        (if (Widget|IsVisible _wbp_inventory)
          (Input|SetInputModeGameandUI self _wbp_gameplay "LockOnCapture" true true)
          (Variables|Default|SetbShowMouseCursor true)
          (Default|BindListenAction _wbp_gameplay "Inventory")))
      (:else))))

(fn ConstructionScript)

(fn CheckLocJson
  (bind _returnvalue (Class|BPlayerController|GetRegionsAroundPlayer))
  (for _array_element _returnvalue
    (if (not (Utilities|Array|ContainsItem (Variables|Default|GetRegionName_Map) _array_element))
      (CallFunction|SVGetDataARegion _array_element))))

(fn CheckLocAssets
  (bind _gltf_manager (Variables|Default|GetGLTF_Manager))
  (bind (_x _y) (Class|BPlayerController|GetRegionPlayer))
  (if (not (Utilities|Array|ContainsItem (Variables|Default|GetRegionName_Assets) (Utilities|String|Append (Utilities|String|ToString(Integer) _x) "_" (Utilities|String|ToString(Integer) _y))))
    (Utilities|Array|AddUnique (Variables|Default|GetRegionName_Assets) (Utilities|String|Append (Utilities|String|ToString(Integer) _x) "_" (Utilities|String|ToString(Integer) _y)))
    (bind _returnvalue (Class|GLTFSpawnManager|SVGetAssetsARegionSendtoClient _gltf_manager (Utilities|String|Append (Utilities|String|ToString(Integer) _x) "_" (Utilities|String|ToString(Integer) _y))))
    (bind _outassets (Class|GLTFSpawnManager|GetAssetsNotEmpty _returnvalue))
    (CallFunction|OCCheckLoadAssets (Utilities|String|Append (Utilities|String|ToString(Integer) _x) "_" (Utilities|String|ToString(Integer) _y)) (Utilities|Struct|BreakChunkAssets _outassets))
    (Default|SVLoadRegionAssets _gltf_manager (Utilities|String|Append (Utilities|String|ToString(Integer) _x) "_" (Utilities|String|ToString(Integer) _y)) _outassets)))

(fn GetPlayerNamefromClient
  (bind _asbp_bgame_instance (Utilities|Casting|CastToBP_BGameInstance (Game|GetGameInstance)))
  (CallFunction|SVSetPlayerData (Variables|/Game/Blueprints/GameMode/BP_BGameInstance.BP_BGameInstance_C|GetPlayerData _asbp_bgame_instance))
  (return))

(fn SetOwnerLight
  (params (bNewOnlyOwnerSee :type Boolean))
  (bind _outactors (Actor|GetAllActorsOfClass "/Game/Blueprints/Light/BP_SV_Light.BP_SV_Light_C"))
  (for _array_element _outactors
    (if (Utilities|Enum|Equal(Enum) (Variables|/Game/Blueprints/Light/BP_SV_Light.BP_SV_Light_C|GetOwnerName _array_element) (PlayerState|GetPlayerName (Variables|Default|GetPlayerState)))
      (for _array_element_2 (Actor|GetComponentsByClass _array_element "/Script/Engine.StaticMeshComponent")
        (Rendering|SetOnlyOwnerSee _array_element_2 bNewOnlyOwnerSee :!class /Script/Engine.PrimitiveComponent)))))

(fn SetOwnerLight0
  (params (NewOwner :type Actor%20Object%20Reference))
  (bind _outactors (Actor|GetAllActorsOfClass "/Game/Blueprints/Light/BP_SV_Light.BP_SV_Light_C"))
  (for _array_element _outactors
    (if (Utilities|Enum|Equal(Enum) (Variables|/Game/Blueprints/Light/BP_SV_Light.BP_SV_Light_C|GetOwnerName _array_element) (PlayerState|GetPlayerName (Variables|Default|GetPlayerState)))
      (Actor|SetOwner _array_element NewOwner))))

(fn SVSetMaterialColor
  (params (BP_AsyncGLTF :type BP%20Async%20GLTF%20Spawn%20Object%20Reference) (Colors :type Array%20of%20Color%20Materials%20Structures))
  (bind (_data _returnvalue) (Class|GLTFSpawnManager|SetMaterialColorGLTF (Variables|Default|GetGLTF_Manager) (Variables|/Game/Blueprints/Actor_Base/BP_Async_GLTF_Spawn.BP_Async_GLTF_Spawn_C|GetRegion BP_AsyncGLTF) (Variables|/Game/Blueprints/Actor_Base/BP_Async_GLTF_Spawn.BP_Async_GLTF_Spawn_C|GetGLTF_Name BP_AsyncGLTF) Colors (Variables|/Game/Blueprints/Actor_Base/BP_Async_GLTF_Spawn.BP_Async_GLTF_Spawn_C|GetIndex BP_AsyncGLTF)))
  (if _returnvalue
    (Default|MCCallSetMaterialColor BP_AsyncGLTF Colors)))

(fn FirstLoc
  (bind (_x _y) (Class|BPlayerController|GetRegionPlayer))
  (if (not (Utilities|Array|ContainsItem (Variables|Default|GetRegionName_Map) (Utilities|String|Append (Utilities|String|ToString(Integer) _x) "_" (Utilities|String|ToString(Integer) _y))))
    (CallFunction|SVGetDataARegion (Utilities|String|Append (Utilities|String|ToString(Integer) _x) "_" (Utilities|String|ToString(Integer) _y)))))