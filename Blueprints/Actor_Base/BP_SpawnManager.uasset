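; Networked spawn manager for runtime glTF assets, lights and client placement previews.
; The server polls an asset list; its RepNotify preloads assets on the server and syncs icon widgets on clients.
; glTFRuntime downloads assets from a port 3000 host into a name-keyed cache feeding spawn events.
; Saved region data spawns glTF actors or tag-configured lights once per region, while clients spawn an editable actor under the mouse cursor.
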(event Custom|Reset_Read
  (bind _outs (|ReadListFileAsync (Variables|Default|GetUrl))
    (:Completed
      (if (!= (Variables|Default|GetLength) (Utilities|Array|Length _outs))
        (Variables|Default|SetLength (Utilities|Array|Length _outs))
        (Variables|Default|SetServer_GLTF_Asset _outs)))))

(event Custom|CustomEvent_2
  (params (Asset :type Gl%20TF%20Runtime%20Asset%20Object%20Reference))
  (bind _runtimecontextstring (Variables|/Script/glTFRuntime.glTFRuntimeAsset|GetRuntimeContextString Asset))
  (Utilities|IsValid Asset
    (:Is%20Valid
      (Utilities|Map|Add (Variables|Default|GetGLTF_List) _runtimecontextstring Asset)
      (CallFunction|CallSpawnGltf (stale Custom|MC_Spawn_GLTF Location) _runtimecontextstring))))

(event Custom|CustomEvent
  (params (Asset :type Gl%20TF%20Runtime%20Asset%20Object%20Reference))
  (bind _runtimecontextstring (Variables|/Script/glTFRuntime.glTFRuntimeAsset|GetRuntimeContextString Asset))
  (Utilities|IsValid Asset
    (:Is%20Valid
      (Utilities|Map|Add (Variables|Default|GetGLTF_List) _runtimecontextstring Asset)
      (CallFunction|CallSpawnGltf (stale Custom|Spawn_GLTF Location) _runtimecontextstring))))

(event Custom|Spawn_GLTF
  (params (Name :type String) (Location :type Transform))
  (if (.ReturnValue (Utilities|Map|Find (Variables|Default|GetGLTF_List) Name))
    (CallFunction|CallSpawnGltf Location Name)
    (else
      (bind _asbp_bgame_instance (Utilities|Casting|CastToBP_BGameInstance (Game|GetGameInstance)))
      (Class|GlTFRuntimeFunctionLibrary|GlTFLoadAssetfromUrl (Utilities|String|ToString(Text) (Utilities|Text|FormatText "{ip}:3000/{name}" (Utilities|String|SelectString "localhost" (Variables|/Game/Blueprints/GameMode/BP_BGameInstance.BP_BGameInstance_C|GetIP _asbp_bgame_instance) (Networking|IsServer)) Name)) 0 (delegate Custom|CustomEvent) (Utilities|Struct|MakeglTFRuntimeConfig Name "node")))))

(event Custom|MC_Spawn_GLTF
  (params (Name :type String) (Location :type Transform))
  (if (Utilities|Map|Contains (Variables|Default|GetGLTF_List) Name)
    (CallFunction|CallSpawnGltf Location Name)
    (else
      (bind _asbp_bgame_instance (Utilities|Casting|CastToBP_BGameInstance (Game|GetGameInstance)))
      (Class|GlTFRuntimeFunctionLibrary|GlTFLoadAssetfromUrl (Utilities|String|ToString(Text) (Utilities|Text|FormatText "{ip}:3000/{name}" (Utilities|String|SelectString "localhost" (Variables|/Game/Blueprints/GameMode/BP_BGameInstance.BP_BGameInstance_C|GetIP _asbp_bgame_instance) (Networking|IsServer)) Name)) 0 (delegate Custom|CustomEvent_2) (Utilities|Struct|MakeglTFRuntimeConfig Name "node")))))

(event Custom|CompletedLoadAsset
  (params (Asset :type Gl%20TF%20Runtime%20Asset%20Object%20Reference))
  (Utilities|IsValid Asset
    (:Is%20Valid
      (Utilities|Map|Add (Variables|Default|GetGLTF_List) (Variables|/Script/glTFRuntime.glTFRuntimeAsset|GetRuntimeContextString Asset) Asset))))

(event Custom|SV_LoadRegionAssets
  (params (RegionName :type String%20%28by%20ref%29) (Assets :type Chunk%20Assets%20Structure))
  (bind (_name _assets) (Utilities|Struct|BreakChunkAssets Assets))
  (if (not (Utilities|Map|Contains (Variables|Default|GetSV_Region_Assets) RegionName))
    (Utilities|Map|Add (Variables|Default|GetSV_Region_Assets) RegionName Assets)
    (for (_array_element _array_index) _name
      (if (.ReturnValue (Utilities|String|Split _array_element ":"))
        (bind _outslot (Class|GLTFSpawnManager|GetAssetNotEmptySendtoClient (Utilities|Array|Get(acopy) _assets _array_index)))
        (for _array_element_2 _outslot
          (switch string (.RightS (Utilities|String|Split _array_element ":"))
            (:Light
              (bind _data (Class|BLibrary|ConvertCompoundTagstoData (.data (Utilities|Array|Get(acopy) (.Tags (Utilities|Struct|BreakChunkAssetsChild (Utilities|Array|Get(acopy) _assets _array_index))) _array_element_2))))
              (for _array_element_3 _data
                (switch string (.Name (Utilities|Struct|BreakCompountTags2 _array_element_3))
                  (:B:Light
                    (bind (_typenum _new_intensity _attenuation_radius _source_radius _enable _new_light_color) (CallFunction|SetLightValues (.TagValue (Utilities|Struct|BreakCompountTags2 _array_element_3)))))))
              (Game|SpawnActorfromClass "/Game/Blueprints/Light/BP_SV_Light.BP_SV_Light_C" (Utilities|Array|Get(acopy) (.Transform (Utilities|Struct|BreakChunkAssetsChild (Utilities|Array|Get(acopy) _assets _array_index))) _array_element_2) "Undefined" 0 _typenum _new_intensity _attenuation_radius _source_radius _enable _new_light_color RegionName _array_element_2 (Utilities|Struct|BreakAsset_Info (Utilities|Array|Get(acopy) (.Info (Utilities|Struct|BreakChunkAssetsChild (Utilities|Array|Get(acopy) _assets _array_index))) _array_element_2)) 0))))
        (else
          (bind _outslot_2 (Class|GLTFSpawnManager|GetAssetNotEmptySendtoClient (Utilities|Array|Get(acopy) _assets _array_index)))
          (for _array_element_4 _outslot_2
            (bind _data_2 (Class|BLibrary|ConvertCompoundTagstoData (Utilities|Struct|BreakCompountContainer (Utilities|Array|Get(acopy) (.Tags (Utilities|Struct|BreakChunkAssetsChild (Utilities|Array|Get(acopy) _assets _array_index))) _array_element_4))))
            (bind _returnvalue (Game|SpawnActorfromClass "/Game/Blueprints/Actor_Base/BP_Async_GLTF_Spawn.BP_Async_GLTF_Spawn_C" (Utilities|Array|Get(acopy) (.Transform (Utilities|Struct|BreakChunkAssetsChild (Utilities|Array|Get(acopy) _assets _array_index))) _array_element_4) "Undefined" 0 self RegionName RegionName _array_element_4 (Utilities|Array|Get(acopy) (.Info (Utilities|Struct|BreakChunkAssetsChild (Utilities|Array|Get(acopy) _assets _array_index))) _array_element_4) (Utilities|Struct|MakeCompountContainer2 _data_2) 0))
            (Variables|/Game/Blueprints/Actor_Base/BP_Async_GLTF_Spawn.BP_Async_GLTF_Spawn_C|SetGLTF_Name _returnvalue _array_element)))))))

(event Custom|Load_WidgetAssets
  ;[1 0.1408 0] Load Widget
  (Variables|Default|GetWG
    (:then
      _)
    (:else
      (bind _foundwidgets (Widget|GetAllWidgetsOfClass "/Game/Blueprints/Widgets/WBP_GamePlay.WBP_GamePlay_C" true :!label _label))
      (if (Utilities|Array|IsNotEmpty _foundwidgets)
        (Utilities|IsValid (Utilities|Array|Get(acopy) _foundwidgets)
          (:Is%20Valid
            (Variables|Default|Setwg_GamePlay (Utilities|Array|Get(acopy) _foundwidgets))
            (Variables|Default|SetWG (Variables|/Game/Blueprints/Widgets/RTTM_Widget.RTTM_Widget_C|GetWBP_AssetIconList (Variables|/Game/Blueprints/Widgets/WBP_GamePlay.WBP_GamePlay_C|GetRTTM_Widget (Utilities|Array|Get(acopy) _foundwidgets)))))
          (:Is%20Not%20Valid
            (Utilities|FlowControl|Delay 0.2 :!label _label_2)
            (goto _label)))
        (else
          (goto _label_2)))))
  (for (_array_element _array_index) (Variables|Default|GetServer_GLTF_Asset)
    (bind _has (CallFunction|CheckWidget _array_element))
    (if (not _has)
      (bind _returnvalue (UserInterface|CreateWidget "/Game/Blueprints/Widgets/WBP_AssetIcon.WBP_AssetIcon_C" 0 _array_element (Utilities|Text|ToText(String) (.LeftS (Utilities|String|Split _array_element "."))) _array_index))
      (Class|WrapBox|AddChildtoWrapBox (Variables|/Game/Blueprints/Widgets/WBP_AssetIconList.WBP_AssetIconList_C|GetWrapBox_List (Variables|Default|GetWG)) _returnvalue)))
  (CallFunction|CheckWidgettoRemove))

(event Custom|Check_LoadAsset_GLTF
  (params (RegionName :type String%20%28by%20ref%29) (Arrays :type Array%20of%20Strings))
  ;[1 0 0.436] Check_LoadAsset_GLTF
  (if (not (Utilities|Array|IsEmpty RegionName))
    (for _array_element Arrays
      (if (not (Utilities|Map|Contains (Variables|Default|GetGLTF_List) _array_element))
        (Class|GlTFRuntimeFunctionLibrary|GlTFLoadAssetfromUrl (Utilities|String|ToString(Text) (Utilities|Text|FormatText "{ip}:3000/{name}" (Variables|/Game/Blueprints/GameMode/BP_BGameInstance.BP_BGameInstance_C|GetIP (.AsBP%20BGame%20Instance (Utilities|Casting|CastToBP_BGameInstance (Game|GetGameInstance)))) _array_element)) 0 (delegate Custom|add) (Utilities|Struct|MakeglTFRuntimeConfig _array_element))))))

(event Custom|CL_Spawn_gltf
  (params (Name :type String%20%28by%20ref%29))
  (bind _gltf_list (Variables|Default|GetGLTF_List))
  (bind (_value _returnvalue) (Utilities|Map|Find _gltf_list Name))
  (Variables|Default|GetBP_Async_Edit
    (:then)
    (:else
      (if _returnvalue
        (CallFunction|GLTFSpawnerManagerAutoGenFunc _value)
        (else
          (bind _asbp_bgame_instance (Utilities|Casting|CastToBP_BGameInstance (Game|GetGameInstance)))
          (Class|GlTFRuntimeFunctionLibrary|GlTFLoadAssetfromUrl (Utilities|String|ToString(Text) (Utilities|Text|FormatText "{ip}:3000/{name}" (Variables|/Game/Blueprints/GameMode/BP_BGameInstance.BP_BGameInstance_C|GetIP _asbp_bgame_instance) Name)) 0 (delegate Custom|CustomEvent_0) (Utilities|Struct|MakeglTFRuntimeConfig Name)))))))

(event Custom|SV_LoadAssets
  (for _array_element (Variables|Default|GetServer_GLTF_Asset)
    (if (not (and (Utilities|IsValid (.Value (Utilities|Map|Find (Variables|Default|GetGLTF_List) _array_element))) (.ReturnValue (Utilities|Map|Find (Variables|Default|GetGLTF_List) _array_element))))
      (Class|GlTFRuntimeFunctionLibrary|GlTFLoadAssetfromUrl (Utilities|String|ToString(Text) (Utilities|Text|FormatText "localhost:3000/{name}" _array_element)) 0 (delegate Custom|CompletedLoadAsset) (Utilities|Struct|MakeglTFRuntimeConfig _array_element)))))

(event Custom|CustomEvent_0
  (params (Asset :type Gl%20TF%20Runtime%20Asset%20Object%20Reference))
  (Utilities|IsValid Asset
    (:Is%20Valid
      (Utilities|Map|Add (Variables|Default|GetGLTF_List) (Variables|/Script/glTFRuntime.glTFRuntimeAsset|GetRuntimeContextString Asset) Asset)
      (CallFunction|GLTFSpawnerManagerAutoGenFunc Asset))))

(event Custom|SV%20Spawn%20GLTF
  (params (Name :type String%20%28by%20ref%29) (Region :type String) (Transform :type Transform) (Index :type Integer) (Info :type Asset%20Info%20Structure) (Data :type Compount%20Container%202%20Structure))
  (bind _returnvalue (Game|SpawnActorfromClass "/Game/Blueprints/Actor_Base/BP_Async_GLTF_Spawn.BP_Async_GLTF_Spawn_C" Transform "AlwaysSpawn" 0 self Region Region Index Info Data 0))
  (Variables|/Game/Blueprints/Actor_Base/BP_Async_GLTF_Spawn.BP_Async_GLTF_Spawn_C|SetGLTF_Name _returnvalue Name))

(event Custom|add
  (params (Asset :type Gl%20TF%20Runtime%20Asset%20Object%20Reference))
  ;[1 0 0.436] Check_LoadAsset_GLTF
  (Utilities|IsValid Asset
    (:Is%20Valid
      (Utilities|Map|Add (Variables|Default|GetGLTF_List) (Variables|/Script/glTFRuntime.glTFRuntimeAsset|GetRuntimeContextString Asset) Asset))))

(event EventBeginPlay
  (Utilities|FlowControl|Delay 5.0)
  (if (Networking|IsServer)
    (Utilities|Time|SetTimerbyFunctionName 0 "Reset_Read" 1.0 true 1.0)))

(fn ConstructionScript)

(fn OnRepServerGLTFAsset
  (if (Networking|IsServer)
    (CallFunction|SVLoadAssets)
    (else
      (CallFunction|LoadWidgetAssets))))

(fn CheckWidget
  (params (Name :type String))
  (for _array_element (Class|PanelWidget|GetAllChildren (Variables|/Game/Blueprints/Widgets/WBP_AssetIconList.WBP_AssetIconList_C|GetWrapBox_List (Variables|Default|GetWG)))
    (bind _aswbp_asset_icon (Utilities|Casting|CastToWBP_AssetIcon _array_element))
    (if (Utilities|Enum|Equal(Enum) (Variables|/Game/Blueprints/Widgets/WBP_AssetIcon.WBP_AssetIcon_C|GetAssetName _aswbp_asset_icon) Name)
      (return true)))
  (return false))

(fn CheckWidgettoRemove
  (for _array_element (Class|PanelWidget|GetAllChildren (Variables|/Game/Blueprints/Widgets/WBP_AssetIconList.WBP_AssetIconList_C|GetWrapBox_List (Variables|Default|GetWG)))
    (bind _aswbp_asset_icon (Utilities|Casting|CastToWBP_AssetIcon _array_element))
    (if (not (Utilities|Array|ContainsItem (Variables|Default|GetServer_GLTF_Asset) (Variables|/Game/Blueprints/Widgets/WBP_AssetIcon.WBP_AssetIcon_C|GetAssetName _aswbp_asset_icon)))
      (Widget|RemovefromParent _aswbp_asset_icon))))

(fn CallSpawnGltf
  (params (SpawnTransform :type Transform) (GLTF_Name :type String))
  (bind _returnvalue (Game|SpawnActorfromClass :Class "/Game/Blueprints/Actor_Base/BP_Async_GLTF_Spawn.BP_Async_GLTF_Spawn_C" :SpawnTransform SpawnTransform :CollisionHandlingOverride "Undefined" :GLTF_Spawner self :Instigator 0))
  (Variables|/Game/Blueprints/Actor_Base/BP_Async_GLTF_Spawn.BP_Async_GLTF_Spawn_C|SetGLTF_Name _returnvalue GLTF_Name))

(fn GLTFSpawnerManagerAutoGenFunc
  (params (Asset :type Gl%20TF%20Runtime%20Asset%20Object%20Reference))
  (bind _returnvalue (Game|GetPlayerController 0))
  (Utilities|IsValid Asset
    (:Is%20Valid
      (bind _location (CallFunction|GetMouseLocation0))
      (bind _returnvalue_2 (Game|SpawnActorfromClass :Class "/Game/Blueprints/Actor_Base/BP_Async_GLTF_Edit.BP_Async_GLTF_Edit_C" :SpawnTransform (Math|Transform|MakeTransform _location "0, 0, 0" "1.000000,1.000000,1.000000") :CollisionHandlingOverride "AlwaysSpawn" :Owner _returnvalue :Name (Variables|/Script/glTFRuntime.glTFRuntimeAsset|GetRuntimeContextString Asset) :Asset Asset :StaticMeshConfig (Utilities|Struct|MakeglTFRuntimeStaticMeshConfig "None" false true false 0 0 "CTF_UseSimpleAndComplex" false "Asset" 0 (Utilities|Struct|MakeglTFRuntimeMaterialsConfig "ReadWrite" "Opaque") 0 "" 0 "IfMissing" "IfMissing" false false false false 0 0) :Instigator 0))
      (Input|EnableInput _returnvalue_2 _returnvalue)
      (Variables|Default|SetBP_Async_Edit _returnvalue_2)
      (Default|ShowOutLine _returnvalue_2))))

(fn DestroyEditGLTF
  (bind _bp_async_edit (Variables|Default|GetBP_Async_Edit)
    (:then
      (Actor|DestroyActor _bp_async_edit))
    (:else)))

(fn GetMouseLocation0
  (bind _returnvalue (Class|WidgetLayoutLibrary|GetViewportScale))
  (bind _returnvalue_2 (Class|WidgetLayoutLibrary|GetMousePositiononViewport))
  (bind (_outhit _returnvalue_3) (Collision|LineTraceByChannel (.WorldPosition (Class|GameplayStatics|DeprojectScreentoWorld (Game|GetPlayerController 0) (* _returnvalue_2 (Math|Vector2D|MakeVector2D _returnvalue _returnvalue)))) (+ (.WorldPosition (Class|GameplayStatics|DeprojectScreentoWorld (Game|GetPlayerController 0) (* _returnvalue_2 (Math|Vector2D|MakeVector2D _returnvalue _returnvalue)))) (* (.WorldDirection (Class|GameplayStatics|DeprojectScreentoWorld (Game|GetPlayerController 0) (* _returnvalue_2 (Math|Vector2D|MakeVector2D _returnvalue _returnvalue)))) 2e+04)) "TraceTypeQuery3" false 0 "None"))
  (if _returnvalue_3
    (return (.Location (Collision|BreakHitResult _outhit)))))

(fn SetLightValues
  (params (Values :type Array%20of%20Strings))
  (for (_array_element _array_index) Values
    (switch int _array_index
      (:0
        (LocalVariables|SetT (Math|Conversions|ToInteger(Byte) _array_element)))
      (:1
        (LocalVariables|SetI (Math|Conversions|ToFloat(Integer) _array_element)))
      (:2
        (LocalVariables|SetA (Math|Conversions|ToFloat(Integer) _array_element)))
      (:3
        (LocalVariables|SetS (Math|Conversions|ToFloat(Integer) _array_element)))
      (:4
        (LocalVariables|SetE (Utilities|Enum|Equal(Enum) _array_element "true")))
      (:5
        (if (.OutIsValid (Math|Conversions|ToColor(LinearColor) _array_element))
          (LocalVariables|SetL (.OutConvertedColor (Math|Conversions|ToColor(LinearColor) _array_element)))))))
  (return (LocalVariables|GetT) (LocalVariables|GetI) (LocalVariables|GetA) (LocalVariables|GetS) (LocalVariables|GetE) (LocalVariables|GetL)))