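; BP_CheckSnap is a helper actor that mirrors another actor's static meshes and reports what it overlaps, apparently for snap checking.
; Init adds a component per source static mesh, copying only the mesh asset, with manual attachment and the source ignored during movement.
; It then attaches itself to that actor, snapping location and rotation.
; A begin-overlap handler bound at BeginPlay only prints the other actor's name.
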(event Custom|OnActorBeginOverlap_Event
  (params (OverlappedActor :type Actor%20Object%20Reference) (OtherActor :type Actor%20Object%20Reference))
  (Development|PrintString (Utilities|GetDisplayName OtherActor)))

(event EventBeginPlay
  (EventDispatchers|BindEventtoOnActorBeginOverlap (delegate Custom|OnActorBeginOverlap_Event)))

(fn ConstructionScript)

(fn Init
  (params (Actor :type Actor%20Object%20Reference))
  (bind _returnvalue (Actor|GetComponentsByClass Actor "/Script/Engine.StaticMeshComponent"))
  (if (Utilities|Array|IsValidIndex _returnvalue)
    (for _array_element _returnvalue
      (bind _returnvalue_2 (Game|AddComponentbyClass "/Script/Engine.StaticMeshComponent" true))
      (Components|StaticMesh|SetStaticMesh _returnvalue_2 (Variables|/Script/Engine.StaticMeshComponent|GetStaticMesh _array_element))
      (Collision|IgnoreActorwhenMoving _returnvalue_2 Actor true))
    (Transformation|AttachActorToActor Actor "None" "SnapToTarget" "SnapToTarget" "KeepRelative" true)))