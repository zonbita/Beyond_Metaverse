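; BP_Actor_DownTris is a hexagon-set actor that leaves a destruction actor behind when it is destroyed.
; On BeginPlay it binds to its own OnDestroyed event, which disables collision and spawns Actor_Destruct_BOT at the same rotation and scale, offset downward in Z.
; The construction script fills the ACNFT AssetInfo with the object name, a random integer and fixed values, so the random number re-rolls whenever construction runs.
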(event Custom|OnDestroyed_Event
  (params (DestroyedActor :type Actor%20Object%20Reference))
  (bind _returnvalue (Transformation|GetActorTransform DestroyedActor))
  (Utilities|IsValid DestroyedActor
    (:Is%20Valid
      (Collision|SetActorEnableCollision DestroyedActor false)
      (Game|SpawnActorfromClass "/Game/Blueprints/Actor_Base/Hexagon/Actor_Destruct_BOT.Actor_Destruct_BOT_C" (Math|Transform|MakeTransform (Math|Vector|MakeVector (.x (.location _returnvalue)) (.y (.location _returnvalue)) (- (.z (.location _returnvalue)) 2.2e+02)) (.rotation _returnvalue) (.scale _returnvalue)) "AlwaysSpawn" 0 0))))

(event EventBeginPlay
  (Game|AssignOnDestroyed (delegate Custom|OnDestroyed_Event)))

(fn ConstructionScript
  (Variables|/Script/BeyondOnline2.AC_NFT|SetAsset_Info (Variables|Default|GetAC_NFT) (Utilities|Struct|MakeAsset_Info (Utilities|GetObjectName self) "" 0.0 (Math|Random|RandomInteger 353534) 6)))