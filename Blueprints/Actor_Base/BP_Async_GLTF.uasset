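; Base actor for an asynchronously loaded glTF asset with recolorable materials and selection-style outlines.
; On load it flags GLTFManager complete and parses "Material:" data tags into a Colors array; on error it destroys itself.
; SetColorMaterial matches components by name, takes materials from the first DT_MaterialTableList table, and sets baseColorFactor on dynamic instances.
; Outline functions toggle custom depth on static meshes, varying stencil values with IsMoving.
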(event OnError(Asset)
  (params (ErrorContext :type String) (ErrorMessage :type String))
  (bind _gltf_manager (Variables|Default|GetGLTF_Manager)
    (:then
      (Variables|/Script/BeyondOnline2.GLTF_SpawnManager|SetLoad_Complete _gltf_manager true)
      (Actor|DestroyActor))
    (:else)))

(event EventOnScenesLoaded
  (bind _gltf_manager (Variables|Default|GetGLTF_Manager)
    (:then
      (Variables|/Script/BeyondOnline2.GLTF_SpawnManager|SetLoad_Complete _gltf_manager true)
      (CallFunction|InitMaterialColor))
    (:else)))

(fn ConstructionScript
  (Variables|/Script/BeyondOnline2.AC_NFT|SetAsset_Info (Variables|Default|GetAC_NFT) (Variables|Default|GetInfo)))

(fn InitMaterialColor
  (for _array_element (.data (Variables|Default|GetData))
    (if (and (Utilities|Enum|Equal(Enum) (.LeftS (Utilities|String|Split (.name _array_element) ":")) "Material") (.ReturnValue (Utilities|String|Split (.name _array_element) ":")))
      (bind (_tableindex _rowname _color_) (CallFunction|LGetMaterialColor (.tagvalue _array_element)))
      (Utilities|Array|Add (Variables|Default|GetColors) (Utilities|Struct|MakeColorMaterials (.name _array_element) _tableindex _rowname _color_))))
  (if (Utilities|Array|IsNotEmpty (Variables|Default|GetColors))
    (CallFunction|SetColorMaterial)))

(fn AddColorMaterial
  (params (NewItem :type Color%20Materials%20Structure%20%28by%20ref%29))
  (bind _colors (Variables|Default|GetColors))
  (bind (_array_element _array_index) (Utilities|Array|ForEachLoopwithBreak (Variables|Default|GetColors) :!label _label)
    (:LoopBody
      (if (Utilities|Enum|Equal(Enum) (.componnentname _array_element) (Utilities|Struct|BreakColorMaterials NewItem))
        (LocalVariables|SetIndex _array_index)
        (goto _label Break)))
    (:Completed
      (if (!= (LocalVariables|GetIndex) -1)
        (Utilities|Array|SetArrayElem _colors (LocalVariables|GetIndex) NewItem)
        (else
          (Utilities|Array|Add _colors NewItem))))))

(fn SetColorMaterial
  (LocalVariables|SetComp (Actor|GetComponentsByClass "/Script/Engine.PrimitiveComponent"))
  (for _array_element (Variables|Default|GetColors)
    (for _array_element_2 (LocalVariables|GetComp)
      (if (Utilities|Enum|Equal(Enum) (Utilities|GetObjectName _array_element_2) (.RightS (Utilities|String|Split (.componnentname _array_element) ":")))
        (if (not (Utilities|Array|IsEmpty (Utilities|String|ToString(Name) (.rowname _array_element))))
          (bind _outrownames (DataTable|GetDataTableRowNames "/Game/Blueprints/MaterialList/DT_MaterialTableList.DT_MaterialTableList"))
          (bind _returnvalue (Utilities|GetDataTableRow "/Game/Blueprints/MaterialList/DT_MaterialTableList.DT_MaterialTableList" (Utilities|Array|Get(acopy) _outrownames))
            (:then
              (bind _returnvalue_2 (Utilities|GetDataTableRow (.table _returnvalue) (.rowname _array_element))
                (:then
                  (Utilities|IsValid (Rendering|Material|GetMaterial _array_element_2 0)
                    (:Is%20Valid
                      (bind _returnvalue_3 (Rendering|Material|CreateDynamicMaterialInstance (Utilities|Struct|BreakS_MaterialList _returnvalue_2) "None" "None" :!class /Script/Engine.KismetMaterialLibrary))
                      (bind _output_get (LocalVariables|SetM_instance _returnvalue_3))
                      (Rendering|Material|SetMaterial _array_element_2 0 _output_get)
                      (bind _m_instance (LocalVariables|GetM_instance)
                        (:then
                          (Rendering|Material|SetVectorParameterValue _m_instance "baseColorFactor" (.color _array_element) :!class /Script/Engine.MaterialInstanceDynamic))
                        (:else)))))))))))))

(fn FindSetColor
  (params (Name :type String) (Item%20Color :type Linear%20Color%20Structure))
  (bind _colors (Variables|Default|GetColors))
  (bind (_array_element _array_index) (Utilities|Array|ForEachLoopwithBreak _colors :!label _label)
    (:LoopBody
      (if (Utilities|Enum|Equal(Enum) (.componnentname _array_element) Name)
        (LocalVariables|Setb (Utilities|Enum|Equal(Enum) (.componnentname _array_element) Name))
        (Utilities|Array|SetArrayElem _colors _array_index (Utilities|Struct|MakeColorMaterials (.componnentname _array_element) (.tableindex _array_element) (.rowname _array_element) Item%20Color))
        (goto _label Break)))
    (:Completed
      (if (not (LocalVariables|Getb))
        (Utilities|Array|AddUnique (Variables|Default|GetColors) (Utilities|Struct|MakeColorMaterials Name 0 "None" Item%20Color))))))

(fn OutLine
  (params (bValue :type Boolean))
  (bind _returnvalue (Actor|GetComponentsByClass "/Script/Engine.StaticMeshComponent"))
  (if bValue
    (if (Variables|Default|GetisMoving)
      (for _array_element _returnvalue
        (bind _asprimitive_component (Utilities|Casting|CastToPrimitiveComponent _array_element))
        (Rendering|SetRenderCustomDepth _asprimitive_component bValue)
        (Rendering|SetCustomDepthStencilValue _asprimitive_component 3)))
    (else
      (Variables|Default|SetisMoving false)
      (for _array_element_2 _returnvalue
        (bind _asprimitive_component_2 (Utilities|Casting|CastToPrimitiveComponent _array_element_2))
        (Rendering|SetRenderCustomDepth _asprimitive_component_2 false)))))

(fn InitOutLine
  (if (not (Variables|Default|GetisMoving))
    (for _array_element (Actor|GetComponentsByClass "/Script/Engine.StaticMeshComponent")
      (bind _asprimitive_component (Utilities|Casting|CastToPrimitiveComponent _array_element))
      (Rendering|SetRenderCustomDepth _asprimitive_component true)
      (Rendering|SetCustomDepthStencilValue _asprimitive_component 0))))