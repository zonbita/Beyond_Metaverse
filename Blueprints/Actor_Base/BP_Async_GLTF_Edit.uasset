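; BP_Async_GLTF_Edit is an actor Blueprint, apparently for editing async-loaded glTF models, that supports outline highlighting and a save-time widget.
; OutLine toggles custom depth rendering on every static mesh component and sets a fixed stencil value, presumably for a post-process outline.
; The ShowOutLine event turns the outline on.
; Reset passes a time value to the WBP_SaveTime instance in its Widget component.
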(event Custom|ShowOutLine
  (CallFunction|OutLine true))

(fn ConstructionScript)

(fn OutLine
  (params (bValue :type Boolean))
  (for _array_element (Actor|GetComponentsByClass "/Script/Engine.StaticMeshComponent")
    (bind _asprimitive_component (Utilities|Casting|CastToPrimitiveComponent _array_element))
    (Rendering|SetRenderCustomDepth _asprimitive_component bValue)
    (Rendering|SetCustomDepthStencilValue _asprimitive_component 3)))

(fn Reset
  (params (Time :type Integer))
  (bind _aswbp_save_time (Utilities|Casting|CastToWBP_SaveTime (UserInterface|GetWidget (Variables|Default|GetWidget))))
  (Default|Reset _aswbp_save_time Time))