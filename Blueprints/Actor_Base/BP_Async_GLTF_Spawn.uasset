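; Replicated placeholder actor that spawns a runtime glTF model as an attached BP_Async_GLTF actor when its GLTF name replicates.
; Spawn retries each frame until the GLTFSpawner is free and has the named asset, then clears its LoadComplete flag as a lock so loads run one at a time.
; Transform and color events pass changes on to the child, with the server storing colors, and destruction removes the child.
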(event Custom|Spawn
  (bind _self self)
  (bind _gltf_spawner (Variables|Default|GetGLTF_Spawner)
    (:then
      (if (Variables|/Script/BeyondOnline2.GLTF_SpawnManager|GetLoad_Complete _gltf_spawner)
        (if (Utilities|IsValid (.Value (Utilities|Map|Find (Variables|/Script/BeyondOnline2.GLTF_SpawnManager|GetGLTF_List _gltf_spawner) (Variables|Default|GetGLTF_Name))))
          (if (Variables|/Script/BeyondOnline2.GLTF_SpawnManager|GetLoad_Complete _gltf_spawner)
            (Variables|/Script/BeyondOnline2.GLTF_SpawnManager|SetLoad_Complete _gltf_spawner false)
            (bind _returnvalue (Game|SpawnActorfromClass :Class "/Game/Blueprints/Actor_Base/BP_Async_GLTF.BP_Async_GLTF_C" :CollisionHandlingOverride "AlwaysSpawn" :Owner _self :GLTF_Manager (Variables|Default|GetGLTF_Spawner) :GLTF_Spawn _self :Info (Variables|Default|GetInfo) :Data (Variables|Default|GetData) :Colors (Variables|Default|GetColors) :Asset (.Value (Utilities|Map|Find (Variables|/Script/BeyondOnline2.GLTF_SpawnManager|GetGLTF_List _gltf_spawner) (Variables|Default|GetGLTF_Name))) :StaticMeshConfig (Utilities|Struct|MakeglTFRuntimeStaticMeshConfig "ReadWrite" false true false 0 0 "CTF_UseSimpleAndComplex" false "Asset" 0 (Utilities|Struct|MakeglTFRuntimeMaterialsConfig "ReadWrite" "Opaque") 0 "" 0 "IfMissing" "IfMissing" false false false false 0 0) :Instigator 0))
            (bind _output_get (Variables|Default|SetGLTF _returnvalue))
            (Transformation|AttachActorToActor _output_get self "None" "KeepRelative" "KeepRelative" "KeepRelative" true)
            (else
              (Utilities|FlowControl|Delay (Utilities|Time|GetWorldDeltaSeconds) :!label _label)
              (CallFunction|Spawn)))
          (else
            (goto _label)))
        (else
          (goto _label))))
    (:else
      (goto _label))))

(event Custom|MC_Call_Set_Material_Color
  (params (Colors :type Array%20of%20Color%20Materials%20Structures))
  (Utilities|FlowControl|Sequence
    (:then_0
      (bind _gltf (Variables|Default|GetGLTF)
        (:then
          (Variables|/Game/Blueprints/Actor_Base/BP_Async_GLTF.BP_Async_GLTF_C|SetColors _gltf Colors)
          (Default|SetColorMaterial _gltf))
        (:else)))
    (:then_1
      (if (Networking|IsServer)
        (Variables|Default|SetColors Colors)))))

(event Custom|MC_Call_Transform
  (params (Transform :type Transform))
  (Transformation|SetActorTransform Transform)
  (bind _gltf (Variables|Default|GetGLTF)
    (:then
      (Transformation|SetActorTransform _gltf Transform false true))
    (:else)))

(event EventDestroyed
  (bind _gltf (Variables|Default|GetGLTF)
    (:then
      (Actor|DestroyActor _gltf))
    (:else)))

(fn ConstructionScript)

(fn OnRepGLTFName
  (CallFunction|Spawn))