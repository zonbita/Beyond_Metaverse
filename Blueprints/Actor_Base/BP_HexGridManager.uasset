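; Server-side manager that builds the hex grid world map and periodically saves its chunks.
; On BeginPlay it reads the map size from the server config file, spawns a random-spawn manager, then calls CreateMap.
; Each OnChunkSpawned callback spawns an attached chunk manager, passing it the region data, meshes and spawn manager.
; A looping timer tells every chunk manager in the world to save once a minute.
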(event Custom|OnChunkSpawned_Event
  (params (RegionData :type Region%20Data%20Structure) (Transform :type Transform) (OwnerChunk :type String))
  (bind _self self)
  (bind _returnvalue (Game|SpawnActorfromClass "/Game/Blueprints/Actor_Base/BPChunkManager.BPChunkManager_C" Transform "Undefined" _self RegionData OwnerChunk (Utilities|Struct|BreakRegionData RegionData) (Variables|Default|GetArray%20Mesh) (Variables|Default|GetSpawnRandomManager) _self 0))
  (Transformation|AttachActorToActor _returnvalue self "None" "KeepRelative" "KeepRelative" "KeepRelative" true))

(event Custom|SaveChunk
  (bind _outactors (Actor|GetAllActorsOfClass "/Game/Blueprints/Actor_Base/BPChunkManager.BPChunkManager_C"))
  (for _array_element _outactors
    (Utilities|IsValid _array_element
      (:Is%20Valid
        (Default|SaveChunk _array_element)))))

(event EventBeginPlay
  (if (Networking|IsServer)
    (CallFunction|Init)
    (Utilities|FlowControl|Sequence
      (:then_0
        (bind _returnvalue (Game|SpawnActorfromClass "/Script/BeyondOnline2.SpawnRandomManager" (Math|Transform|MakeTransform "0, 0, 0" "0, 0, 0" "1.000000,1.000000,1.000000") "Undefined" 0 self 0))
        (Variables|Default|SetSpawnRandomManager _returnvalue))
      (:then_1
        (EventDispatchers|AssignOnChunkSpawned (delegate Custom|OnChunkSpawned_Event)))
      (:then_2
        (Class|HexGridManager|CreateMap (Variables|Default|GetSize) 6))
      (:then_3
        (if (Networking|IsServer)
          (Utilities|Time|SetTimerbyFunctionName 0 "SaveChunk" 6e+01 true))))))

(fn ConstructionScript)

(fn Init
  (bind _configdata (Class|HexGridManager|LoadConfigfromFile "ServerConfig.cfg"))
  (bind _keys (Utilities|Map|Keys _configdata))
  (bind _values (Utilities|Map|Values _configdata))
  (for (_array_element _array_index) _keys
    (switch string _array_element
      (:ConfigSize
        (Variables|Default|SetSize (Math|Conversions|ToInteger(Byte) (Utilities|Array|Get(acopy) _values _array_index)))))))