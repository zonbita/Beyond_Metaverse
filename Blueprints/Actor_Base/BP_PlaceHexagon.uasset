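; BP_PlaceHexagon is a triangle mesh actor that stores a triangle name, chunk and up/down orientation, and requests hexagon placement from the player controller.
; Set stores those values and picks the up or bottom triangle mesh.
; CallToPC splits the name into parts, adjusts two by orientation (incrementing the third for down triangles), then passes the rebuilt name and data to BP_BPlayerController's PlaceHexagon.
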(fn ConstructionScript)

(fn Set
  (params (Up :type Boolean) (Name :type String) (Chunk_ :type BP%20Chunk%20Manager%20Object%20Reference))
  (bind _output_get (Variables|Default|SetUp Up))
  (Variables|Default|SetTriangleName Name)
  (Variables|Default|SetChunk Chunk_)
  (Components|StaticMesh|SetStaticMesh (Variables|Debug|GetStaticMeshComponent) (select _output_get "/Game/Blueprints/Actor_Base/Hexagon/DestructionTri/Tri4_UpTri_Tri4_UpTri.Tri4_UpTri_Tri4_UpTri" "/Game/Blueprints/Actor_Base/Hexagon/DestructionTri/Tri4_BotTri_Tri4_BOTTri.Tri4_BotTri_Tri4_BOTTri")))

(fn CalltoPC
  (bind _up (Variables|Default|GetUp))
  (bind _asbp_bplayer_controller (Utilities|Casting|CastToBP_BPlayerController (Game|GetPlayerController 0)))
  (bind _returnvalue (Class|BLibrary|GetAllValueOfTriangleName (Variables|Default|GetTriangleName)))
  (bind _returnvalue_2 (Class|BLibrary|ConvertArraytoTriangleName (Utilities|Array|MakeArray (Utilities|Array|Get(acopy) _returnvalue) (Utilities|Array|Get(acopy) _returnvalue 1) (Utilities|String|SelectString (Utilities|Array|Get(acopy) _returnvalue 2) (Utilities|String|ToString(Integer) (+ (Math|Conversions|ToInteger(Byte) (Utilities|Array|Get(acopy) _returnvalue 2)) 1)) _up) (Utilities|Array|Get(acopy) _returnvalue 3) (Utilities|String|SelectString "a" (Utilities|Array|Get(acopy) _returnvalue 4) _up))))
  (Default|PlaceHexagon _asbp_bplayer_controller _returnvalue_2 (Variables|Default|GetChunk) (Utilities|Array|MakeArray (Utilities|Array|Get(acopy) _returnvalue) (Utilities|Array|Get(acopy) _returnvalue 1) (Utilities|String|SelectString (Utilities|Array|Get(acopy) _returnvalue 2) (Utilities|String|ToString(Integer) (+ (Math|Conversions|ToInteger(Byte) (Utilities|Array|Get(acopy) _returnvalue 2)) 1)) _up) (Utilities|Array|Get(acopy) _returnvalue 3) (Utilities|String|SelectString "a" (Utilities|Array|Get(acopy) _returnvalue 4) _up)) (Variables|Default|GetUp)))