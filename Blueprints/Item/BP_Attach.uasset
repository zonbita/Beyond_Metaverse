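; BP_Attach is an item actor that shows a data table entry as a static mesh held in the player character's right hand.
; Init runs at construction and BeginPlay, reading the configured row to set the item's name and mesh.
; With a BP_BPlayerController owner, it caches the controller and its BP_ThirdPersonCharacter, then snaps to that character's hand_r socket.
; An invalid table only prints an error.
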(event EventBeginPlay
  (CallFunction|Init))

(fn ConstructionScript
  (CallFunction|Init))

(fn Init
  (bind _returnvalue (Components|GetOwner))
  (bind _table (Variables|Default|GetTable))
  (Utilities|IsValid (.datatable _table)
    (:Is%20Valid
      (bind _returnvalue_2 (Utilities|GetDataTableRow (.datatable _table) (.rowname _table))
        (:then
          (Utilities|FlowControl|Sequence
            (:then_0
              (Variables|Default|SetName (Utilities|String|ToString(Text) (.Name (Utilities|Struct|BreakS_Item__Info _returnvalue_2))))
              (if (Utilities|IsValid (.SM (Utilities|Struct|BreakS_Item__Info _returnvalue_2)))
                (Components|StaticMesh|SetStaticMesh (Variables|Default|GetSM) (.SM (Utilities|Struct|BreakS_Item__Info _returnvalue_2)))))
            (:then_1
              (Utilities|IsValid _returnvalue
                (:Is%20Valid
                  (bind _asbp_bplayer_controller (Utilities|Casting|CastToBP_BPlayerController _returnvalue))
                  (bind _output_get (Variables|Default|SetBP%20BPlayer%20Controller _asbp_bplayer_controller))
                  (bind _asbp_third_person_character (Utilities|Casting|CastToBP_ThirdPersonCharacter (Pawn|GetControlledPawn _output_get)))
                  (bind _output_get_2 (Variables|Default|SetBP%20Third%20Person%20Character _asbp_third_person_character))
                  (Transformation|AttachComponentToComponent (Variables|/Script/Engine.Character|GetMesh _output_get_2) "hand_r" "SnapToTarget" "SnapToTarget" "KeepRelative" true))))))))
    (:Is%20Not%20Valid
      (Development|PrintString (Utilities|String|Append "Error not found table" (Utilities|String|ToString(Name) (.rowname _table)))))))