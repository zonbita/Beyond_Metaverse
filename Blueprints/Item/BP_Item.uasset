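; BP_Item is a world item actor that a player can pick up into their inventory.
; On BeginPlay it reads its data table row to set its name and static mesh, copying the row's attributes only when Default is set.
; The ITakeItem interface event passes the attributes to the player controller's inventory component and destroys the actor on success.
; A Taking flag blocks re-entrant pickups and resets on failure.
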(event EventITakeItem
  (params (PC :type Player%20Controller%20Object%20Reference))
  (if (not (Variables|Default|GetTaking))
    (Variables|Default|SetTaking true)
    (bind _asbp_bplayer_controller (Utilities|Casting|CastToBP_BPlayerController PC)
      (:then
        (bind _add (Default|AddItem (Variables|/Game/Blueprints/GameMode/BP_BPlayerController.BP_BPlayerController_C|GetBP_AC_Inventory_Player _asbp_bplayer_controller) (Variables|Default|GetItem_Attribte)))
        (if _add
          (Actor|DestroyActor)
          (else
            (Variables|Default|SetTaking false))))
      (:CastFailed
        (Variables|Default|SetTaking false)))))

(event EventBeginPlay
  (CallFunction|Init))

(fn ConstructionScript)

(fn Init
  (bind _table (Variables|Default|GetTable))
  (Utilities|IsValid (.datatable _table)
    (:Is%20Valid
      (bind _returnvalue (Utilities|GetDataTableRow (.datatable _table) (.rowname _table))
        (:then
          (Variables|Default|SetName (Utilities|String|ToString(Text) (.Name (Utilities|Struct|BreakS_Item__Info _returnvalue))))
          (if (Variables|Default|GetDefault)
            (Variables|Default|SetItem_Attribte (.Attribute (Utilities|Struct|BreakS_Item__Info _returnvalue))))
          (Utilities|FlowControl|Sequence
            (:then_0
              (if (Utilities|IsValid (.SM (Utilities|Struct|BreakS_Item__Info _returnvalue)))
                (Components|StaticMesh|SetStaticMesh (Variables|Default|GetSM) (.SM (Utilities|Struct|BreakS_Item__Info _returnvalue)))))))))
    (:Is%20Not%20Valid
      (Development|PrintString (Utilities|String|Append "Error not found table" (Utilities|String|ToString(Name) (.rowname _table)))))))