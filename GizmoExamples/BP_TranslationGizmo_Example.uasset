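; Translation gizmo that attaches to BP_Async_GLTF actors, toggling their outline and highlighting the hovered or active handle by swapping materials, restoring cached originals afterwards.
; Gizmo state changes flag the parent as moving and, for plane drags only, run a looping timer that box-traces its bounds.
; The first blocking hit after each reset is latched, and Tick holds the actor at that Y-adjusted point as a simple collision snap.
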(event Custom|CustomEvent
  (params (GizmoType :type ETransformationType%20Enum :default "TT_NoTransform") (bTransformInProgress :type Boolean) (CurrentDomain :type ETransformationDomain%20Enum :default "TD_None"))
  (bind _returnvalue (Actor|GetAttachParentActor))
  (Variables|Default|SetCurrent%20Domain CurrentDomain)
  (Utilities|FlowControl|Sequence
    (:then_0
      (Utilities|IsValid (Variables|Default|GetSelected%20Mesh)
        (:Is%20Valid
          (Utilities|FlowControl|Sequence
            (:then_0
              (for _index (range 0 (- (Rendering|Material|GetNumMaterials (Variables|Default|GetSelected%20Mesh)) 1))
                (Rendering|Material|SetMaterial (Variables|Default|GetSelected%20Mesh) _index (Utilities|Array|Get(acopy) (CallFunction|GetMaterialArray (Utilities|Array|FindItem (Variables|Default|GetArrayMesh) (Variables|Default|GetSelected%20Mesh))) _index))))
            (:then_1
              (switch Utilities|FlowControl|Switch|SwitchonETransformationDomain CurrentDomain :!label _label
                (:TD_X_Axis
                  (Variables|Default|SetSelected%20Mesh (Variables|Default|GetX_Mesh)))
                (:TD_Y_Axis
                  (Variables|Default|SetSelected%20Mesh (Variables|Default|GetY_Mesh)))
                (:TD_Z_Axis
                  (Variables|Default|SetSelected%20Mesh (Variables|Default|GetZ_Mesh)))
                (:TD_XY_Plane
                  (Variables|Default|SetSelected%20Mesh (Variables|Default|GetXY_Mesh)))
                (:TD_YZ_Plane
                  (Variables|Default|SetSelected%20Mesh (Variables|Default|GetYZ_Mesh)))
                (:TD_XZ_Plane
                  (Variables|Default|SetSelected%20Mesh (Variables|Default|GetXZ_Mesh)))
                (:TD_XYZ
                  (Variables|Default|SetSelected%20Mesh (Variables|Default|GetXYZ_Mesh))))
              (for _index_2 (range 0 (- (Rendering|Material|GetNumMaterials (Variables|Default|GetSelected%20Mesh)) 1))
                (Rendering|Material|SetMaterial (Variables|Default|GetSelected%20Mesh) _index_2 (Variables|Default|GetMaterial%20for%20Selection))))))
        (:Is%20Not%20Valid
          (goto _label))))
    (:then_1
      (if (Utilities|Enum|NotEqual(Enum) (Variables|Default|GetCurrent%20Domain) "TD_None")
        (Utilities|FlowControl|Sequence
          (:then_0
            (Utilities|IsValid _returnvalue
              (:Is%20Valid
                (bind _asbp_async_gltf (Utilities|Casting|CastToBP_Async_GLTF _returnvalue))
                (bind _output_get (Variables|Default|SetAs%20BP%20Async%20GLTF _asbp_async_gltf))
                (Variables|/Game/Blueprints/Actor_Base/BP_Async_GLTF.BP_Async_GLTF_C|SetisMoving _output_get true)
                (Default|OutLine _output_get true))))
          (:then_1
            (switch Utilities|FlowControl|Switch|SwitchonETransformationDomain (Variables|Default|GetCurrent%20Domain)
              (:TD_None
                (Utilities|Time|PauseTimerbyHandle (Variables|Default|GetTimer_Check) :!label _label_2))
              (:TD_X_Axis
                (goto _label_2))
              (:TD_Y_Axis
                (goto _label_2))
              (:TD_Z_Axis
                (goto _label_2))
              (:TD_XY_Plane
                (Variables|Default|GetAs%20BP%20Async%20GLTF :!label _label_3
                  (:then
                    (CallFunction|Reset)
                    (Utilities|Time|UnpauseTimerbyHandle (Variables|Default|GetTimer_Check)))
                  (:else)))
              (:TD_YZ_Plane
                (goto _label_3))
              (:TD_XZ_Plane
                (goto _label_3))
              (:TD_XYZ
                (goto _label_2)))))
        (else
          (Utilities|Time|PauseTimerbyHandle (Variables|Default|GetTimer_Check))
          (Variables|Default|SetAs%20BP%20Async%20GLTF 0)
          (Variables|Default|SetHit%20Actor 0))))))

(event Custom|Check
  ;[1 1 1] Comment
  (bind _as_bp_async_gltf (Variables|Default|GetAs%20BP%20Async%20GLTF)
    (:then
      (bind (_outhit _returnvalue) (Class|KismetSystemLibrary|BoxTraceSingleforObjects (.Origin (Collision|GetActorBounds _as_bp_async_gltf false false)) (.Origin (Collision|GetActorBounds _as_bp_async_gltf false false)) (.BoxExtent (Collision|GetActorBounds _as_bp_async_gltf false false)) (Transformation|GetActorRotation _as_bp_async_gltf) (Utilities|Array|MakeArray "ObjectTypeQuery1" "ObjectTypeQuery2") false (Utilities|Array|MakeArray (Variables|Default|GetAs%20BP%20Async%20GLTF)) "None" true))
      (if _returnvalue
        (if (.bBlockingHit (Collision|BreakHitResult _outhit))
          (Utilities|FlowControl|DoOnce false
            (:Completed
              (Variables|Default|SetImpact%20Point (Math|Vector|MakeVector (.x (.Location (Collision|BreakHitResult _outhit))) (- (.y (.Location (Collision|BreakHitResult _outhit))) (* (.y (.Normal (Collision|BreakHitResult _outhit))) 2.0)) (.z (.Location (Collision|BreakHitResult _outhit)))))
              (Variables|Default|SetHit%20Actor (.HitActor (Collision|BreakHitResult _outhit))))))))
    (:else)))

(event Custom|Reset
  ;[1 1 1] Comment
  (Utilities|FlowControl|DoOnce false) ; enters at Reset
)

(event EventBeginPlay
  (Utilities|FlowControl|Sequence
    (:then_0
      (CallFunction|SetDefaultMaterial)
      (bind _returnvalue (Utilities|Time|SetTimerbyFunctionName 0 "Check" 0.01 true))
      (bind _output_get (Variables|Default|SetTimer_Check _returnvalue))
      (Utilities|Time|PauseTimerbyHandle _output_get)
      (EventDispatchers|AssignOnGizmoStateChange (delegate Custom|CustomEvent)))))

(event EventTick
  (params (DeltaSeconds :type Float%20%28single-precision%29))
  (bind _returnvalue (Actor|GetAttachParentActor))
  ;[1 1 1] Comment
  (Utilities|FlowControl|Sequence
    (:then_0
      (bind _returnvalue_2 (Transformation|AttachComponentToComponent (Variables|Default|GetRootScene) (Transformation|GetAttachParent (Variables|Default|GetRootScene)) "None" "SnapToTarget" "SnapToTarget" "SnapToTarget" false))
      (if _returnvalue_2
        (Utilities|FlowControl|DoOnce false :!label _label
          (:Completed
            (Utilities|IsValid _returnvalue
              (:Is%20Valid
                (bind _asbp_async_gltf (Utilities|Casting|CastToBP_Async_GLTF _returnvalue))
                (Default|InitOutLine _asbp_async_gltf)))))
        (else
          (goto _label Reset))))
    (:then_1
      (Utilities|FlowControl|Delay DeltaSeconds)
      (switch Utilities|FlowControl|Switch|SwitchonETransformationDomain (Variables|Default|GetCurrent%20Domain)
        (:TD_XY_Plane
          _)
        (:TD_YZ_Plane
          _)
        (:TD_XZ_Plane
          _))
      (bind _hit_actor (Variables|Default|GetHit%20Actor)
        (:then
          (bind _as_bp_async_gltf (Variables|Default|GetAs%20BP%20Async%20GLTF)
            (:then
              (Transformation|SetActorLocation _as_bp_async_gltf (Variables|Default|GetImpact%20Point) false true))
            (:else)))
        (:else)))))

(event EventSelectHighlight
  (params (Component :type Primitive%20Component%20Object%20Reference))
  ;[1 1 1] Comment
  (Utilities|IsValid Component
    (:Is%20Valid
      (if (not (== Component (Variables|Default|GetTarget)))
        (bind _target (Variables|Default|GetTarget)
          (:then
            (bind _asstatic_mesh_component (Utilities|Casting|CastToStaticMeshComponent (Components|GetChildComponent _target 0)))
            (for (_array_element _array_index) (CallFunction|GetMaterialArray (Utilities|Array|FindItem (Variables|Default|GetArrayMesh) _asstatic_mesh_component))
              (Rendering|Material|SetMaterial _asstatic_mesh_component _array_index _array_element)))
          (:else
            _))
        (Variables|Default|SetTarget Component)
        (Variables|Default|GetTarget
          (:then
            (bind _asstatic_mesh_component_2 (Utilities|Casting|CastToStaticMeshComponent (Components|GetChildComponent (Variables|Default|GetTarget) 0)))
            (for (_ _array_index_2) (Rendering|Material|GetMaterials _asstatic_mesh_component_2)
              (Rendering|Material|SetMaterial _asstatic_mesh_component_2 _array_index_2 (Variables|Default|GetMaterial%20for%20Selection))))
          (:else))))
    (:Is%20Not%20Valid
      (bind _target_2 (Variables|Default|GetTarget)
        (:then
          (bind _asstatic_mesh_component_3 (Utilities|Casting|CastToStaticMeshComponent (Components|GetChildComponent _target_2 0)))
          (for (_array_element_2 _array_index_3) (CallFunction|GetMaterialArray (Utilities|Array|FindItem (Variables|Default|GetArrayMesh) _asstatic_mesh_component_3))
            (Rendering|Material|SetMaterial _asstatic_mesh_component_3 _array_index_3 _array_element_2))
          (Variables|Default|SetTarget 0))
        (:else)))))

(event EventDestroyed
  (bind _returnvalue (Actor|GetAttachParentActor))
  ;[1 1 1] Comment
  (Utilities|IsValid _returnvalue
    (:Is%20Valid
      (bind _asbp_async_gltf (Utilities|Casting|CastToBP_Async_GLTF _returnvalue))
      (if (not (Variables|/Game/Blueprints/Actor_Base/BP_Async_GLTF.BP_Async_GLTF_C|GetisMoving _asbp_async_gltf))
        (Default|OutLine _asbp_async_gltf false)))))

(fn ConstructionScript)

(fn SetDefaultMaterial
  (bind _output_get (Variables|Default|SetArrayMesh (Utilities|Array|MakeArray (Variables|Default|GetXZ_Mesh) (Variables|Default|GetXYZ_Mesh) (Variables|Default|GetYZ_Mesh) (Variables|Default|GetXY_Mesh) (Variables|Default|GetZ_Mesh) (Variables|Default|GetY_Mesh) (Variables|Default|GetX_Mesh))))
  (for (_array_element _array_index) _output_get
    (switch int _array_index
      (:0
        (Variables|Default|SetXZ (Rendering|Material|GetMaterials _array_element)))
      (:1
        (Variables|Default|SetXYZ (Rendering|Material|GetMaterials _array_element)))
      (:2
        (Variables|Default|SetYZ (Rendering|Material|GetMaterials _array_element)))
      (:3
        (Variables|Default|SetXY (Rendering|Material|GetMaterials _array_element)))
      (:4
        (Variables|Default|SetZ (Rendering|Material|GetMaterials _array_element)))
      (:5
        (Variables|Default|SetY (Rendering|Material|GetMaterials _array_element)))
      (:6
        (Variables|Default|SetX (Rendering|Material|GetMaterials _array_element))))))

(fn GetMaterialArray
  (params (Index :type Integer))
  (return (Utilities|Select :Index Index :Option%200 (Variables|Default|GetXZ) :Option%201 (Variables|Default|GetXYZ) :Option%202 (Variables|Default|GetYZ) :Option%203 (Variables|Default|GetXY) :Option%204 (Variables|Default|GetZ) :Option%205 (Variables|Default|GetY) :Option%206 (Variables|Default|GetX))))